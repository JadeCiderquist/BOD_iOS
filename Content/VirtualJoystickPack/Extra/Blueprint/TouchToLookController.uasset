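; Example touch-to-look controller from the Virtual Joystick Pack that rotates the view by dragging on the right half of the screen.
; The first touch caches half the viewport width, avoiding a zero value on mobile.
; Each press stores its finger index, and right-side presses also capture start position and control rotation.
; Right-side moves add the halved drag offset to that captured rotation, setting pitch and yaw with zero roll.
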(event EventBeginPlay
  ;[1 1 1] This is unused in this example.
)

(event Input|TouchEvents|InputTouch
  (params (Location :type Vector) (FingerIndex :type ETouchIndex%20Enum))
  (:Pressed
    (Utilities|FlowControl|Sequence
      (:then_0
        ;[1 1 1] We want to get the half screen size on first touch only.
        ; This to avoid the RightScreenSize value returning 0
        ; on mobile.
        (Utilities|FlowControl|DoOnce false
          (:Completed
            (Variables|Default|SetRightScreenSize (/ (Math|Conversions|ToFloat(Integer) (.SizeX (HUD|GetViewportSize))) 2.0)))))
      (:then_1
        ;[1 1 1] Setting this variable simply helps
        ; the controller to choose which
        ; finger index to use when player
        ; use the virtual joystick and the
        ; engine registered it as touch 1, which
        ; on that case, this var will be set
        ; to touch 2, and touch 1 otherwise
        (Variables|Default|SetFingerIndexToUse FingerIndex)
        (if (> (.X (Math|Vector|BreakVector Location)) (Variables|Default|GetRightScreenSize))
          (Variables|Default|SetTouchStarts (Math|Vector2D|MakeVector2D (.LocationX (Class|PlayerController|GetInputTouchState (Variables|Default|GetFingerIndexToUse))) (.LocationY (Class|PlayerController|GetInputTouchState (Variables|Default|GetFingerIndexToUse)))))
          (Variables|Default|SetCapturedRotation (Pawn|GetControlRotation (Game|GetPlayerCharacter 0) :!class /Script/Engine.Pawn))))))
  (:Moved
    (if (> (.X (Math|Vector|BreakVector Location)) (Variables|Default|GetRightScreenSize))
      (Variables|Default|SetTouchEnds (Math|Vector2D|MakeVector2D (.LocationX (Class|PlayerController|GetInputTouchState (Variables|Default|GetFingerIndexToUse))) (.LocationY (Class|PlayerController|GetInputTouchState (Variables|Default|GetFingerIndexToUse)))))
      (Pawn|SetControlRotation (Math|Rotator|MakeRotator 0.0 (+ (.Pitch (Math|Rotator|BreakRotator (Variables|Default|GetCapturedRotation))) (|(Y/2) (.Y (Math|Vector2D|BreakVector2D (- (Variables|Default|GetTouchStarts) (Variables|Default|GetTouchEnds)))))) (+ (.Yaw (Math|Rotator|BreakRotator (Variables|Default|GetCapturedRotation))) (|((x*y)/2) (.X (Math|Vector2D|BreakVector2D (- (Variables|Default|GetTouchStarts) (Variables|Default|GetTouchEnds)))) -1.0)))) ; Final input
    )))

(fn ConstructionScript)