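; Flying-movement shark enemy for a VR underwater game that bites the player and can be shot dead.
; Sphere overlap starts a looping bite timer paced by montage length, driving sound, haptics, player damage and an underwater material-parameter update.
; Projectile hits on the Box reduce health and shrink the widget bar by resizing its draw size.
; Death plays an animation, slows movement, then ramps a material parameter by timeline before destroying the actor.
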(event `self.ReceiveBeginPlay`
  ;[1 1 1] 血条
)

(event `loop`
  (bind _returnvalue (`GameplayStatics.GetPlayerController` 0))
  ;[1 1 1] 鲨鱼咬人
  (if (not (`self.Death`))
    (bind _returnvalue_2 (`AnimInstance.Montage_Play` (`SkeletalMeshComponent.GetAnimInstance` (`self.Mesh`)) "/Game/Chaunychen/GreatWhiteShark/Animations/Anim_SharkBite_Montage.Anim_SharkBite_Montage" 1.2 "MontageLength" 0.0 true :!label _label))
    (bind _returnvalue_3 (`KismetSystemLibrary.K2_SetTimerDelegate` (delegate `loop`) _returnvalue_2 true))
    (`GameplayStatics.PlaySound2D` "/Game/JadeCiderquist/Sound/Shark_Attack.Shark_Attack" 1.0 1.0 0.0 null null)
    (`PlayerController.PlayHapticEffect` _returnvalue "/Game/JadeCiderquist/Gun/Haptics/SharkEffect.SharkEffect" "Left" 1.0 false)
    (`PlayerController.PlayHapticEffect` _returnvalue "/Game/JadeCiderquist/Gun/Haptics/SharkEffect.SharkEffect" "Right" 1.0 false)
    ;[1 1 1] 角色生命
    (bind _outactors (`GameplayStatics.GetAllActorsOfClass` "/Game/AFCore/Examples/Pawns/VR/BP_Pawn_VR_Char_Example_HandsOn.BP_Pawn_VR_Char_Example_HandsOn_C"))
    (bind _output (`|GetArrayItem` _outactors))
    (if (`/Game/AFCore/Examples/Pawns/VR/BP_Pawn_VR_Char_Example_HandsOn.Do_Death` _output)
      (bind _output_get (set `/Game/AFCore/Examples/Pawns/VR/BP_Pawn_VR_Char_Example_HandsOn.Player_Health` (- (stale _output_get) (/ 1.0 20.0)) _output))
      (`KismetMaterialLibrary.SetScalarParameterValue` "/Game/JadeCiderquist/Material/Underwater/MP_UnderWater.MP_UnderWater" "Xue" (- 1.0 _output_get))
      ;[1 1 1] 手机震动
      (`PlayerController.PlayDynamicForceFeedback` _returnvalue 2.0 0.7 true true true true))))

(event `self.Sphere.OnComponentBeginOverlap`
  (params (OverlappedComponent :type "PrimitiveComponent Object Reference") (OtherActor :type "Actor Object Reference") (OtherComp :type "PrimitiveComponent Object Reference") (OtherBodyIndex :type Integer) (bFromSweep :type Boolean) (SweepResult :type "HitResult Structure (by ref)"))
  ;[1 1 1] 鲨鱼咬人
  (cast `/Game/AFCore/Examples/Pawns/VR/BP_Pawn_VR_Char_Example_HandsOn` OtherActor)
  (if (not (`self.Death`))
    (goto _label)))

(event `self.Sphere.OnComponentEndOverlap`
  (params (OverlappedComponent :type "PrimitiveComponent Object Reference") (OtherActor :type "Actor Object Reference") (OtherComp :type "PrimitiveComponent Object Reference") (OtherBodyIndex :type Integer))
  ;[1 1 1] 玩家远离鲨鱼
  (cast `/Game/AFCore/Examples/Pawns/VR/BP_Pawn_VR_Char_Example_HandsOn` OtherActor)
  (`KismetSystemLibrary.K2_ClearAndInvalidateTimerHandle` (stale `loop` _returnvalue_3)))

(event `self.Box.OnComponentBeginOverlap`
  (params (OverlappedComponent :type "PrimitiveComponent Object Reference") (OtherActor :type "Actor Object Reference") (OtherComp :type "PrimitiveComponent Object Reference") (OtherBodyIndex :type Integer) (bFromSweep :type Boolean) (SweepResult :type "HitResult Structure (by ref)"))
  (bind _charactermovement (`self.CharacterMovement`))
  (bind _comp_widget (`self.Comp_Widget`))
  (bind _death_ani (`self.Death_Ani`))
  (bind (_returnvalue_x _returnvalue_y) (`KismetMathLibrary.BreakVector2D` (`WidgetComponent.GetDrawSize` _comp_widget)))
  ;[1 1 1] 子弹命中
  (bind _asprojectile (cast `/Game/JadeCiderquist/Gun/Blueprints/Projectile` OtherActor))
  (`ActorComponent.Activate` (`/Game/JadeCiderquist/Gun/Blueprints/Projectile.VFX_GrenadeEXP_air` _asprojectile) false)
  ;[1 1 1] 鲨鱼生命
  (bind _output_get (set `self.Health` (- (stale _output_get) (/ (`/Game/JadeCiderquist/Gun/Blueprints/Projectile.Harm` _asprojectile) 3.0))))
  (`WidgetComponent.SetDrawSize` _comp_widget (`KismetMathLibrary.MakeVector2D` (* _returnvalue_x (`self.Health`)) _returnvalue_y))
  ;[1 1 1] 鲨鱼死亡
  (if (<= (`self.Health`) 0.0)
    (`/Engine/EditorBlueprintResources/StandardMacros.DoOnce` false
      (:`Completed`
        (`SkeletalMeshComponent.PlayAnimation` (`self.Mesh`) _death_ani false)
        (set `self.Death` true)
        (bind _returnvalue (`PrimitiveComponent.CreateDynamicMaterialInstance` (`self.Mesh`) 0 "/Game/Chaunychen/GreatWhiteShark/Materials/Mat_GreatWhiteShark_Inst.Mat_GreatWhiteShark_Inst" "None"))
        (set `CharacterMovementComponent.MaxFlySpeed` (/ (`CharacterMovementComponent.MaxFlySpeed` _charactermovement) 3.0) _charactermovement)
        (`KismetSystemLibrary.Delay` (`AnimationAsset.GetPlayLength` _death_ani))
        (bind (_direction `_新建轨道_0`) (`Timeline|时间轴_0`)
          (:`Update`
            (`MaterialInstanceDynamic.SetScalarParameterValue` _returnvalue "Strenth" (`KismetMathLibrary.Lerp` 0.0 1.0 `_新建轨道_0`)))
          (:`Finished`
            (`self.K2_DestroyActor`)))))))

(fn `UserConstructionScript`)