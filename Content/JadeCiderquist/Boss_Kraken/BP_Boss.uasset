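; Kraken boss for the underwater VR fight that turns to track the player and attacks by range.
; A Delay-paced Tick loop plays slam and top/bottom sweep attacks, telegraphed with slow motion and darkening, or spawns ink projectiles at long range.
; Overlap volumes select attacks and toggle Gates controlling damage, haptics and dodge prompts.
; Projectile hits drain its health bar; death dissolves it, reveals the vortex and removes the shield.
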(event `self.ReceiveActorBeginOverlap`
  (params (OtherActor :type "Actor Object Reference"))
  (if (not true)
    ;[1 1 1] 漩涡出现
    (bind _outactors (`GameplayStatics.GetAllActorsOfClass` "/Game/JadeCiderquist/BluePrint/BP_Boss_XuanWo.BP_Boss_XuanWo_C" :!label _label))
    (bind _output (`|GetArrayItem` _outactors))
    (`self.SetActorHiddenInGame` _output false)
    (set `PrimitiveComponent.bGenerateOverlapEvents` true (`/Game/JadeCiderquist/BluePrint/BP_Boss_XuanWo.Sphere` _output))
    (bind (_direction `_新建轨道_0`) (`Timeline|时间轴_5` :!via `PlayFromStart`)
      (:`Update`
        (bind (_color_r _color_g _color_b) (break `LinearColor` (`/Game/JadeCiderquist/BluePrint/BP_Boss_XuanWo.Color` _output)))
        (`NiagaraComponent.SetVariableLinearColor` (`/Game/JadeCiderquist/BluePrint/BP_Boss_XuanWo.NS_Vortex_Boss` _output) "XW_Color" (make `LinearColor` _color_r _color_g _color_b (`KismetMathLibrary.Lerp` 0.0 1.0 `_新建轨道_0`))))
      (:`Finished`
        ;[1 1 1] 保护罩隐藏
        (bind _outactors_2 (`GameplayStatics.GetAllActorsOfClass` "/Game/JadeCiderquist/Circle_Safe/BP_BaoHuZhao.BP_BaoHuZhao_C"))
        (bind _output_2 (`|GetArrayItem` _outactors_2))
        (`PrimitiveComponent.SetCollisionEnabled` (`/Game/JadeCiderquist/Circle_Safe/BP_BaoHuZhao.qiuti_suiji` _output_2) "NoCollision")
        (`self.SetActorHiddenInGame` _output_2 true)))))

(event `self.PaiJi.OnComponentBeginOverlap`
  (params (OverlappedComponent :type "PrimitiveComponent Object Reference") (OtherActor :type "Actor Object Reference") (OtherComp :type "PrimitiveComponent Object Reference") (OtherBodyIndex :type Integer) (bFromSweep :type Boolean) (SweepResult :type "HitResult Structure (by ref)"))
  (bind _returnvalue (`GameplayStatics.GetPlayerController` 0))
  ;[1 1 1] 拍击重叠
  (cast `/Game/AFCore/Examples/Pawns/VR/BP_Pawn_VR_Char_Example_HandsOn` OtherActor)
  ;[1 1 1] 攻击范围文字提示
  (`|ExecutionSequence` :!label _label_2
    (:`then_0`
      (goto _label_5 :!via `Open`))
    (:`then_1`
      (goto _label_6 :!via `Open`))))

(event `self.PaiJi5.OnComponentBeginOverlap`
  (params (OverlappedComponent :type "PrimitiveComponent Object Reference") (OtherActor :type "Actor Object Reference") (OtherComp :type "PrimitiveComponent Object Reference") (OtherBodyIndex :type Integer) (bFromSweep :type Boolean) (SweepResult :type "HitResult Structure (by ref)"))
  ;[1 1 1] 拍击重叠
  (cast `/Game/AFCore/Examples/Pawns/VR/BP_Pawn_VR_Char_Example_HandsOn` OtherActor)
  (goto _label_2))

(event `self.PaiJi2.OnComponentBeginOverlap`
  (params (OverlappedComponent :type "PrimitiveComponent Object Reference") (OtherActor :type "Actor Object Reference") (OtherComp :type "PrimitiveComponent Object Reference") (OtherBodyIndex :type Integer) (bFromSweep :type Boolean) (SweepResult :type "HitResult Structure (by ref)"))
  ;[1 1 1] 拍击重叠
  (cast `/Game/AFCore/Examples/Pawns/VR/BP_Pawn_VR_Char_Example_HandsOn` OtherActor)
  (goto _label_2))

(event `self.PaiJi.OnComponentEndOverlap`
  (params (OverlappedComponent :type "PrimitiveComponent Object Reference") (OtherActor :type "Actor Object Reference") (OtherComp :type "PrimitiveComponent Object Reference") (OtherBodyIndex :type Integer))
  (bind _returnvalue (`GameplayStatics.GetPlayerController` 0))
  ;[1 1 1] 拍击重叠
  (cast `/Game/AFCore/Examples/Pawns/VR/BP_Pawn_VR_Char_Example_HandsOn` OtherActor)
  ;[1 1 1] 攻击范围文字提示
  (`|ExecutionSequence` :!label _label_3
    (:`then_0`
      (goto _label_5 :!via `Close`))
    (:`then_1`
      (bind _outactors (`GameplayStatics.GetAllActorsOfClass` "/Game/AFCore/Examples/Pawns/VR/BP_Pawn_VR_Char_Example_HandsOn.BP_Pawn_VR_Char_Example_HandsOn_C"))
      (bind _output (`|GetArrayItem` _outactors))
      (bind _wbp_bossred (`/Game/AFCore/Examples/Pawns/VR/BP_Pawn_VR_Char_Example_HandsOn.WBP_BOSSred` _output))
      (if (`SceneComponent.IsVisible` _wbp_bossred)
        (`SceneComponent.SetVisibility` _wbp_bossred false false)
        (bind _wbp_bossgreen (`/Game/AFCore/Examples/Pawns/VR/BP_Pawn_VR_Char_Example_HandsOn.WBP_BOSSgreen` _output))
        (`SceneComponent.SetVisibility` _wbp_bossgreen true false)
        (`KismetSystemLibrary.Delay` 2.0)
        (`SceneComponent.SetVisibility` _wbp_bossgreen false false)))
    (:`then_2`
      (goto _label_6 :!via `Close`))))

(event `self.PaiJi5.OnComponentEndOverlap`
  (params (OverlappedComponent :type "PrimitiveComponent Object Reference") (OtherActor :type "Actor Object Reference") (OtherComp :type "PrimitiveComponent Object Reference") (OtherBodyIndex :type Integer))
  ;[1 1 1] 拍击重叠
  (cast `/Game/AFCore/Examples/Pawns/VR/BP_Pawn_VR_Char_Example_HandsOn` OtherActor)
  (goto _label_3))

(event `self.PaiJi2.OnComponentEndOverlap`
  (params (OverlappedComponent :type "PrimitiveComponent Object Reference") (OtherActor :type "Actor Object Reference") (OtherComp :type "PrimitiveComponent Object Reference") (OtherBodyIndex :type Integer))
  ;[1 1 1] 拍击重叠
  (cast `/Game/AFCore/Examples/Pawns/VR/BP_Pawn_VR_Char_Example_HandsOn` OtherActor)
  (goto _label_3))

(event `self.ReceiveTick`
  (params (DeltaSeconds :type "Float (single-precision)"))
  (bind _returnvalue (`GameplayStatics.GetPlayerController` 0))
  (bind _returnvalue_2 (`GameplayStatics.GetPlayerController` 0))
  (bind (_returnvalue_roll _returnvalue_pitch _returnvalue_yaw) (`KismetMathLibrary.BreakRotator` (`self.K2_GetActorRotation`)))
  (bind _returnvalue_3 (`GameplayStatics.GetPlayerController` 0))
  (bind _returnvalue_4 (`self.K2_GetActorLocation`))
  (bind _boss_mat (`self.Boss_MAt`))
  (bind _boss_idle (`self.Boss_idle`))
  (bind _boss_sat (`self.Boss_SAt`))
  (bind _kraken (`self.KRAKEN`))
  (bind _hengsao_bottom (`self.HengSao_Bottom`))
  (bind _boss_satu (`self.Boss_SAtU`))
  (bind _hengsao_up (`self.HengSao_Up`))
  (bind _boss_die (`self.Boss_die`))
  (bind _mouse_sphere (`self.Mouse_Sphere`))
  (bind _returnvalue_5 (* (/ (`self.Ani_Time`) (`self.Time Dilation`)) 1.5))
  (`|ExecutionSequence`
    (:`then_0`
      (`KismetSystemLibrary.Delay` (+ (`self.Ani_Time`) 0.01))
      (if (`self.if_Death`)
        ;[1 1 1] 死亡动画
        (`/Engine/EditorBlueprintResources/StandardMacros.DoOnce` false
          (:`Completed`
            (`SkeletalMeshComponent.PlayAnimation` (`self.KRAKEN`) _boss_die false)
            (`PrimitiveComponent.SetCollisionEnabled` (`self.KRAKEN`) "NoCollision")
            (`KismetSystemLibrary.Delay` (`AnimationAsset.GetPlayLength` _boss_die))
            ;[1 1 1] Noise消散
            (`|ExecutionSequence`
              (:`then_0`
                (`KismetSystemLibrary.Delay` 0.8)
                (`ActorComponent.Activate` (`self.Boss_N`) false)
                (goto _label))
              (:`then_1`
                (bind (_direction `_新建轨道_0`) (`Timeline|时间轴_4`)
                  (:`Update`
                    (`KismetMaterialLibrary.SetScalarParameterValue` "/Game/JadeCiderquist/Boss_Kraken/Materials/MP_Boss.MP_Boss" "Noise_Strenth" (`KismetMathLibrary.Lerp` 0.0 1.0 `_新建轨道_0`))))))))
        (else
          (bind _outactors (`GameplayStatics.GetAllActorsOfClass` "/Game/AFCore/Examples/Pawns/VR/BP_Pawn_VR_Char_Example_HandsOn.BP_Pawn_VR_Char_Example_HandsOn_C"))
          (`|ExecutionSequence`
            (:`then_0`
              (if (`self.if_CloseAttack`)
                (switch `int` (`self.Int_At`)
                  (:`Default`
                    ;[1 1 1] Idle
                    (`SkeletalMeshComponent.PlayAnimation` _kraken _boss_idle false :!label _label_4)
                    (set `self.Ani_Time` (`AnimationAsset.GetPlayLength` _boss_idle))
                    (set `self.Int_At` (`KismetMathLibrary.RandomIntegerInRange` 0 2)))
                  (:`0`
                    ;[1 1 1] 拍打攻击
                    (`|ExecutionSequence`
                      (:`then_0`
                        ;[1 1 1] 攻击范围文字提示
                        (`/Engine/EditorBlueprintResources/StandardMacros.Gate` true :!label _label_5
                          (:`Exit`
                            (bind _outactors_2 (`GameplayStatics.GetAllActorsOfClass` "/Game/AFCore/Examples/Pawns/VR/BP_Pawn_VR_Char_Example_HandsOn.BP_Pawn_VR_Char_Example_HandsOn_C"))
                            (bind _output (`|GetArrayItem` _outactors_2))
                            (bind _wbp_bossred (`/Game/AFCore/Examples/Pawns/VR/BP_Pawn_VR_Char_Example_HandsOn.WBP_BOSSred` _output))
                            (`SceneComponent.SetVisibility` _wbp_bossred true false)
                            (`SceneComponent.SetVisibility` (`/Game/AFCore/Examples/Pawns/VR/BP_Pawn_VR_Char_Example_HandsOn.WBP_BOSSgreen` _output) false false)
                            (`KismetSystemLibrary.Delay` 2.0)
                            (`SceneComponent.SetVisibility` _wbp_bossred false false))))
                      (:`then_1`
                        (set `self.Ani_Time` (`AnimationAsset.GetPlayLength` _boss_mat))
                        (`SceneComponent.SetVisibility` (`self.PaiJi`) true false)
                        (`SceneComponent.SetVisibility` (`self.PaiJi2`) true false)
                        (`SceneComponent.SetVisibility` (`self.PaiJi5`) true false)
                        ;;[0 0.2974 1] 底部横扫攻击
                        (set `self.Int_At` 1)
                        (`GameplayStatics.SetGlobalTimeDilation` (/ 1.0 (`self.Time Dilation`)))
                        (`KismetMaterialLibrary.SetScalarParameterValue` "/Game/JadeCiderquist/Material/Underwater/MP_UnderWater.MP_UnderWater" "Light absorption" 100.0)
                        (`SkeletalMeshComponent.PlayAnimation` _kraken _boss_mat false)
                        (`KismetSystemLibrary.Delay` _returnvalue_5)
                        (`SceneComponent.SetVisibility` (`self.PaiJi`) false false)
                        (`SceneComponent.SetVisibility` (`self.PaiJi2`) false false)
                        (`SceneComponent.SetVisibility` (`self.PaiJi5`) false false)
                        (`KismetMaterialLibrary.SetScalarParameterValue` "/Game/JadeCiderquist/Material/Underwater/MP_UnderWater.MP_UnderWater" "Light absorption" 1.0)
                        (`GameplayStatics.SetGlobalTimeDilation` 1.0)
                        (`KismetSystemLibrary.Delay` 0.5)
                        (`ActorComponent.Activate` (`self.P_FireGroundAttack4`) true)
                        (`ActorComponent.Activate` (`self.P_FireGroundAttack5`) true)
                        (`ActorComponent.Activate` (`self.P_FireGroundAttack3`) true)
                        (`GameplayStatics.PlaySound2D` "/Game/JadeCiderquist/Sound/Kraken_Attack01.Kraken_Attack01" 1.0 1.0 0.0 null null)
                        ;[1 1 1] 命中手柄震动
                        (`/Engine/EditorBlueprintResources/StandardMacros.Gate` true :!label _label_6
                          (:`Exit`
                            (`PlayerController.PlayHapticEffect` _returnvalue "/Game/JadeCiderquist/Gun/Haptics/BossEffect.BossEffect" "Left" 1.0 false)
                            (`PlayerController.PlayHapticEffect` _returnvalue "/Game/JadeCiderquist/Gun/Haptics/BossEffect.BossEffect" "Right" 1.0 false)
                            ;[1 1 1] Test_游戏手柄
                            (`PlayerController.K2_ClientPlayForceFeedback` _returnvalue "/Game/AFCore/Examples/Pawns/VR/Shoubing.Shoubing" "None" false false false)
                            ;[1 1 1] 角色生命
                            (bind _outactors_3 (`GameplayStatics.GetAllActorsOfClass` "/Game/AFCore/Examples/Pawns/VR/BP_Pawn_VR_Char_Example_HandsOn.BP_Pawn_VR_Char_Example_HandsOn_C"))
                            (bind _output_2 (`|GetArrayItem` _outactors_3))
                            (bind _output_get (set `/Game/AFCore/Examples/Pawns/VR/BP_Pawn_VR_Char_Example_HandsOn.Player_Health` (- (stale _output_get) (/ 1.0 3.0)) _output_2))
                            (`KismetMaterialLibrary.SetScalarParameterValue` "/Game/JadeCiderquist/Material/Underwater/MP_UnderWater.MP_UnderWater" "Xue" (- 1.0 _output_get))
                            (if (<= (`/Game/AFCore/Examples/Pawns/VR/BP_Pawn_VR_Char_Example_HandsOn.Player_Health` _output_2) 0.0)
                              (set `self.if_CloseAttack` false)
                              (set `self.if_FarAttack` false)))))))
                  (:`1`
                    ;[1 1 1] 横扫底部攻击
                    (`|ExecutionSequence`
                      (:`then_0`
                        (set `self.Ani_Time` (`AnimationAsset.GetPlayLength` _boss_sat))
                        (`SceneComponent.SetVisibility` _hengsao_bottom true false)
                        (`GameplayStatics.SetGlobalTimeDilation` (/ 1.0 (`self.Time Dilation`)))
                        (`KismetMaterialLibrary.SetScalarParameterValue` "/Game/JadeCiderquist/Material/Underwater/MP_UnderWater.MP_UnderWater" "Light absorption" 100.0)
                        (`SkeletalMeshComponent.PlayAnimation` _kraken _boss_sat false)
                        (`|ExecutionSequence`
                          (:`then_0`
                            ;;[1 0.04098 0] 预警充能
                            (bind (_direction_2 `_新建轨道_0_2`) (`Timeline|时间轴_3` :!via `PlayFromStart`)
                              (:`Update`
                                (`KismetMaterialLibrary.SetScalarParameterValue` "/Game/JadeCiderquist/Boss_Kraken/Materials/MP_Boss.MP_Boss" "Step" (`KismetMathLibrary.Lerp` 0.0 0.2 `_新建轨道_0_2`)))))
                          (:`then_1`
                            (`KismetSystemLibrary.Delay` _returnvalue_5)
                            (`SceneComponent.SetVisibility` _hengsao_bottom false false)
                            (`KismetMaterialLibrary.SetScalarParameterValue` "/Game/JadeCiderquist/Material/Underwater/MP_UnderWater.MP_UnderWater" "Light absorption" 1.0)
                            (`GameplayStatics.SetGlobalTimeDilation` 1.0)
                            (`GameplayStatics.PlaySound2D` "/Game/JadeCiderquist/Sound/Kraken_sweep2.Kraken_sweep2" 1.0 1.0 0.0 null null)
                            ;;[0 0.2974 1] idle
                            (set `self.Int_At` -1)
                            (`KismetSystemLibrary.Delay` 0.5)
                            (`ActorComponent.Activate` (`self.P_GroundAttack`) true)
                            ;[1 1 1] 命中手柄震动
                            (`/Engine/EditorBlueprintResources/StandardMacros.Gate` true :!label _label_7
                              (:`Exit`
                                (`PlayerController.PlayHapticEffect` _returnvalue_3 "/Game/JadeCiderquist/Gun/Haptics/BossEffect.BossEffect" "Left" 1.0 false)
                                (`PlayerController.PlayHapticEffect` _returnvalue_3 "/Game/JadeCiderquist/Gun/Haptics/BossEffect.BossEffect" "Right" 1.0 false)
                                ;[1 1 1] Test_游戏手柄
                                (`PlayerController.K2_ClientPlayForceFeedback` _returnvalue_3 "/Game/AFCore/Examples/Pawns/VR/Shoubing.Shoubing" "None" false false false)
                                ;[1 1 1] 角色生命
                                (bind _outactors_4 (`GameplayStatics.GetAllActorsOfClass` "/Game/AFCore/Examples/Pawns/VR/BP_Pawn_VR_Char_Example_HandsOn.BP_Pawn_VR_Char_Example_HandsOn_C"))
                                (bind _output_3 (`|GetArrayItem` _outactors_4))
                                (bind _output_get_2 (set `/Game/AFCore/Examples/Pawns/VR/BP_Pawn_VR_Char_Example_HandsOn.Player_Health` (- (stale _output_get_2) (/ 1.0 3.0)) _output_3))
                                (`KismetMaterialLibrary.SetScalarParameterValue` "/Game/JadeCiderquist/Material/Underwater/MP_UnderWater.MP_UnderWater" "Xue" (- 1.0 _output_get_2))
                                (if (<= (`/Game/AFCore/Examples/Pawns/VR/BP_Pawn_VR_Char_Example_HandsOn.Player_Health` _output_3) 0.0)
                                  (set `self.if_CloseAttack` false)
                                  (set `self.if_FarAttack` false)))))))
                      (:`then_1`
                        ;[1 1 1] 攻击范围文字提示
                        (`/Engine/EditorBlueprintResources/StandardMacros.Gate` true :!label _label_8
                          (:`Exit`
                            (bind _outactors_5 (`GameplayStatics.GetAllActorsOfClass` "/Game/AFCore/Examples/Pawns/VR/BP_Pawn_VR_Char_Example_HandsOn.BP_Pawn_VR_Char_Example_HandsOn_C"))
                            (bind _output_4 (`|GetArrayItem` _outactors_5))
                            (bind _wbp_bossredup (`/Game/AFCore/Examples/Pawns/VR/BP_Pawn_VR_Char_Example_HandsOn.WBP_BOSSredup` _output_4))
                            (`SceneComponent.SetVisibility` _wbp_bossredup true false)
                            (`SceneComponent.SetVisibility` (`/Game/AFCore/Examples/Pawns/VR/BP_Pawn_VR_Char_Example_HandsOn.WBP_BOSSgreen` _output_4) false false)
                            (`KismetSystemLibrary.Delay` 2.0)
                            (`SceneComponent.SetVisibility` _wbp_bossredup false false))))))
                  (:`2`
                    ;[1 1 1] 横扫顶部攻击
                    (`|ExecutionSequence`
                      (:`then_0`
                        (set `self.Ani_Time` (`AnimationAsset.GetPlayLength` _boss_satu))
                        (`SceneComponent.SetVisibility` _hengsao_up true false)
                        (`GameplayStatics.SetGlobalTimeDilation` (/ 1.0 (`self.Time Dilation`)))
                        (`KismetMaterialLibrary.SetScalarParameterValue` "/Game/JadeCiderquist/Material/Underwater/MP_UnderWater.MP_UnderWater" "Light absorption" 100.0)
                        (`SkeletalMeshComponent.PlayAnimation` _kraken _boss_satu false)
                        (`|ExecutionSequence`
                          (:`then_0`
                            ;;[1 0.04098 0] 预警充能
                            (bind (_direction_3 `_新建轨道_0_3`) (`Timeline|时间轴_2` :!via `PlayFromStart`)
                              (:`Update`
                                (`KismetMaterialLibrary.SetScalarParameterValue` "/Game/JadeCiderquist/Boss_Kraken/Materials/MP_Boss.MP_Boss" "Step" (`KismetMathLibrary.Lerp` 0.0 0.2 `_新建轨道_0_3`)))))
                          (:`then_1`
                            (`KismetSystemLibrary.Delay` (* (/ (`self.Ani_Time`) (`self.Time Dilation`)) 1.5))
                            (`SceneComponent.SetVisibility` _hengsao_up false false)
                            (`KismetMaterialLibrary.SetScalarParameterValue` "/Game/JadeCiderquist/Material/Underwater/MP_UnderWater.MP_UnderWater" "Light absorption" 1.0)
                            (`GameplayStatics.SetGlobalTimeDilation` 1.0)
                            (`GameplayStatics.PlaySound2D` "/Game/JadeCiderquist/Sound/Kraken_sweep2.Kraken_sweep2" 1.0 1.0 0.0 null null)
                            ;;[0 0.2974 1] idle
                            (set `self.Int_At` -1)
                            (`KismetSystemLibrary.Delay` 0.5)
                            (`ActorComponent.Activate` (`self.P_UpAttack`) true)
                            ;[1 1 1] 命中手柄震动
                            (`/Engine/EditorBlueprintResources/StandardMacros.Gate` true :!label _label_9
                              (:`Exit`
                                (`PlayerController.PlayHapticEffect` _returnvalue_2 "/Game/JadeCiderquist/Gun/Haptics/BossEffect.BossEffect" "Left" 1.0 false)
                                (`PlayerController.PlayHapticEffect` _returnvalue_2 "/Game/JadeCiderquist/Gun/Haptics/BossEffect.BossEffect" "Right" 1.0 false)
                                ;[1 1 1] Test_游戏手柄
                                (`PlayerController.K2_ClientPlayForceFeedback` _returnvalue_2 "/Game/AFCore/Examples/Pawns/VR/Shoubing.Shoubing" "None" false false false)
                                ;[1 1 1] 角色生命
                                (bind _outactors_6 (`GameplayStatics.GetAllActorsOfClass` "/Game/AFCore/Examples/Pawns/VR/BP_Pawn_VR_Char_Example_HandsOn.BP_Pawn_VR_Char_Example_HandsOn_C"))
                                (bind _output_5 (`|GetArrayItem` _outactors_6))
                                (bind _output_get_3 (set `/Game/AFCore/Examples/Pawns/VR/BP_Pawn_VR_Char_Example_HandsOn.Player_Health` (- (stale _output_get_3) (/ 1.0 3.0)) _output_5))
                                (`KismetMaterialLibrary.SetScalarParameterValue` "/Game/JadeCiderquist/Material/Underwater/MP_UnderWater.MP_UnderWater" "Xue" (- 1.0 _output_get_3))
                                (if (<= (`/Game/AFCore/Examples/Pawns/VR/BP_Pawn_VR_Char_Example_HandsOn.Player_Health` _output_5) 0.0)
                                  (set `self.if_CloseAttack` false)
                                  (set `self.if_FarAttack` false)))))))
                      (:`then_1`
                        ;[1 1 1] 攻击范围文字提示
                        (`/Engine/EditorBlueprintResources/StandardMacros.Gate` true :!label _label_10
                          (:`Exit`
                            (bind _outactors_7 (`GameplayStatics.GetAllActorsOfClass` "/Game/AFCore/Examples/Pawns/VR/BP_Pawn_VR_Char_Example_HandsOn.BP_Pawn_VR_Char_Example_HandsOn_C"))
                            (bind _output_6 (`|GetArrayItem` _outactors_7))
                            (bind _wbp_bossreddown (`/Game/AFCore/Examples/Pawns/VR/BP_Pawn_VR_Char_Example_HandsOn.WBP_BOSSreddown` _output_6))
                            (`SceneComponent.SetVisibility` _wbp_bossreddown true false)
                            (`SceneComponent.SetVisibility` (`/Game/AFCore/Examples/Pawns/VR/BP_Pawn_VR_Char_Example_HandsOn.WBP_BOSSgreen` _output_6) false false)
                            (`KismetSystemLibrary.Delay` 2.0)
                            (`SceneComponent.SetVisibility` _wbp_bossreddown false false)))))))
                (else
                  (goto _label_4))))
            (:`then_1`
              (bind _returnvalue_6 (`self.K2_GetActorLocation` (`|GetArrayItem` _outactors)))
              (bind _returnvalue_7 (- _returnvalue_6 _returnvalue_4))
              (bind (_returnvalue_x _returnvalue_y) (`KismetMathLibrary.BreakVector` (`KismetMathLibrary.Normal` _returnvalue_7)))
              (set `self.Player_Location` (`KismetMathLibrary.MakeVector` (+ (.x _returnvalue_6) (* _returnvalue_x -3000.0)) (+ (.y _returnvalue_6) (* _returnvalue_y -3000.0)) (.z _returnvalue_4)))
              (set `self.Actor_Location` (`self.K2_GetActorLocation`))
              (`|ExecutionSequence`
                (:`then_0`
                  ;[1 1 1] 计算位移角度
                  (set `self.Rotation_Z` _returnvalue_yaw)
                  (`/Engine/EditorBlueprintResources/StandardMacros.FlipFlop`
                    (:`A`
                      (bind _returnvalue_8 (+ (`KismetMathLibrary.DegAtan2` (.y _returnvalue_7) (.x _returnvalue_7)) 180.0))
                      (bind _output_get_4 (set `self.Player_R01` _returnvalue_8))
                      (bind _returnvalue_9 (- (stale _output_get_5) _output_get_4))
                      (if (< (`KismetMathLibrary.Abs` _returnvalue_9) 180.0)
                        (set `self.Lerp_Pos` _returnvalue_9)
                        (elif (>= _returnvalue_9 0.0)
                          (set `self.Lerp_Pos` (* (+ (- 360.0 (stale _output_get_5)) _output_get_4) -1.0))
                          (else
                            (set `self.Lerp_Pos` (+ _returnvalue_9 360.0))))))
                    (:`B`
                      (bind _output_get_5 (set `self.Player_R02` _returnvalue_8))
                      (bind _returnvalue_10 (- _output_get_4 _output_get_5))
                      (if (< (`KismetMathLibrary.Abs` _returnvalue_10) 180.0)
                        (set `self.Lerp_Pos` _returnvalue_10)
                        (elif (>= _returnvalue_10 0.0)
                          (set `self.Lerp_Pos` (* (+ (- 360.0 _output_get_4) _output_get_5) -1.0))
                          (else
                            (set `self.Lerp_Pos` (+ _returnvalue_10 360.0)))))))
                  (set `self.Rotation_Z_Next` (- (`self.Rotation_Z`) (`self.Lerp_Pos`)))
                  ;[1 1 1] 章鱼旋转
                  (bind (_direction_4 `_新建轨道_0_4`) (`Timeline|时间轴_0` :!via `PlayFromStart`)
                    (:`Update`
                      (`self.K2_SetActorRotation` (`KismetMathLibrary.MakeRotator` 0.0 0.0 (`KismetMathLibrary.Lerp` (`self.Rotation_Z`) (`self.Rotation_Z_Next`) `_新建轨道_0_4`))))))))))))
    (:`then_1`
      ;[1 1 1] 初始旋转角度
      (`/Engine/EditorBlueprintResources/StandardMacros.DoOnce` false
        (:`Completed`
          (bind _outactors_8 (`GameplayStatics.GetAllActorsOfClass` "/Game/AFCore/Examples/Pawns/VR/BP_Pawn_VR_Char_Example_HandsOn.BP_Pawn_VR_Char_Example_HandsOn_C"))
          (`self.K2_SetActorRotation` (`KismetMathLibrary.MakeRotator` 0.0 0.0 (+ (+ (`KismetMathLibrary.DegAtan2` (.y (- (`self.K2_GetActorLocation` (`|GetArrayItem` _outactors_8)) (`self.K2_GetActorLocation`))) (.x (- (`self.K2_GetActorLocation` (`|GetArrayItem` _outactors_8)) (`self.K2_GetActorLocation`)))) 180.0) (`self.Angle_Boss_PianCha`)))))))
    (:`then_2`
      ;[1 1 1] 退出范围停止近战攻击
      (`/Engine/EditorBlueprintResources/StandardMacros.Gate` true :!label _label_11
        (:`Exit`
          (if (`self.Bottom_Attack`)
            _
            (elif (not (`self.Top_Attack`))
              (set `self.if_CloseAttack` false)
              ;[1 1 1] 喷墨水
              (`KismetSystemLibrary.Delay` 1.0)
              (`/Engine/EditorBlueprintResources/StandardMacros.Gate` true :!label _label_12
                (:`Exit`
                  (if (`self.if_Death`)
                    _
                    (elif (`self.if_FarAttack`)
                      (`|SpawnActorFromClass` "/Game/JadeCiderquist/Boss_Kraken/BP_Boss_Mo.BP_Boss_Mo_C" (`KismetMathLibrary.MakeTransform` (`SceneComponent.K2_GetComponentLocation` _mouse_sphere) (`SceneComponent.K2_GetComponentRotation` _mouse_sphere)) "Undefined" "OverrideRootScale" self (`GameplayStatics.GetPlayerPawn` 0)))))))))))))

(event `self.HengSao_Bottom.OnComponentBeginOverlap`
  (params (OverlappedComponent :type "PrimitiveComponent Object Reference") (OtherActor :type "Actor Object Reference") (OtherComp :type "PrimitiveComponent Object Reference") (OtherBodyIndex :type Integer) (bFromSweep :type Boolean) (SweepResult :type "HitResult Structure (by ref)"))
  ;[1 1 1] 底部横扫重叠
  (cast `/Game/AFCore/Examples/Pawns/VR/BP_Pawn_VR_Char_Example_HandsOn` OtherActor)
  (set `self.Bottom_Attack` true)
  (set `self.if_CloseAttack` true)
  ;;[0 0.2974 1] 拍打攻击
  (set `self.Int_At` 0)
  ;[1 1 1] 攻击范围文字提示
  (`|ExecutionSequence`
    (:`then_0`
      (goto _label_7 :!via `Open`))
    (:`then_1`
      (goto _label_8 :!via `Open`))))

(event `self.ReceiveBeginPlay`
  ;[1 1 1] 显示血量
  (`/Game/AFCore/Blueprints/Components/UI/Comp_Widget.SetWidgetVisibility` (`self.Comp_Widget`) true)
  (`/Game/AFCore/Blueprints/Components/UI/Comp_Widget.SetWidgetVisibility` (`self.Comp_Widget1`) true))

(event `self.Attack_FanWei.OnComponentEndOverlap`
  (params (OverlappedComponent :type "PrimitiveComponent Object Reference") (OtherActor :type "Actor Object Reference") (OtherComp :type "PrimitiveComponent Object Reference") (OtherBodyIndex :type Integer))
  ;[1 1 1] 退出范围停止近战攻击
  (cast `/Game/AFCore/Examples/Pawns/VR/BP_Pawn_VR_Char_Example_HandsOn` OtherActor)
  (`|ExecutionSequence`
    (:`then_0`
      (goto _label_11 :!via `Open`))))

(event `self.KRAKEN.OnComponentBeginOverlap`
  (params (OverlappedComponent :type "PrimitiveComponent Object Reference") (OtherActor :type "Actor Object Reference") (OtherComp :type "PrimitiveComponent Object Reference") (OtherBodyIndex :type Integer) (bFromSweep :type Boolean) (SweepResult :type "HitResult Structure (by ref)"))
  (bind _comp_widget (`self.Comp_Widget`))
  (bind (_returnvalue_x _returnvalue_y) (`KismetMathLibrary.BreakVector2D` (`WidgetComponent.GetDrawSize` _comp_widget)))
  ;[1 1 1] 子弹命中整个章鱼
  (bind _asprojectile (cast `/Game/JadeCiderquist/Gun/Blueprints/Projectile` OtherActor))
  (if (not (`self.if_Death`))
    (`ActorComponent.Activate` (`/Game/JadeCiderquist/Gun/Blueprints/Projectile.VFX_GrenadeEXP_air` _asprojectile) false)
    (`GameplayStatics.PlaySound2D` "/Game/JadeCiderquist/Sound/Gun_hit.Gun_hit" 1.0 1.0 0.0 null null)
    ;[1 1 1] 伤害
    (bind _output_get (set `self.Health` (- (stale _output_get) (/ (`/Game/JadeCiderquist/Gun/Blueprints/Projectile.Harm` _asprojectile) 10.0))))
    (`WidgetComponent.SetDrawSize` _comp_widget (`KismetMathLibrary.MakeVector2D` (* 3000.0 (`self.Health`)) _returnvalue_y))
    ;[1 1 1] 死亡设置
    (if (<= (`self.Health`) 0.0) :!label _label_13
      (set `self.if_Death` true)
      (`/Game/AFCore/Blueprints/Components/UI/Comp_Widget.SetWidgetVisibility` (`self.Comp_Widget`) false)
      (`/Game/AFCore/Blueprints/Components/UI/Comp_Widget.SetWidgetVisibility` (`self.Comp_Widget1`) false)
      (`AudioComponent.FadeOut` (`self.BGM`) 5.0 0.0 "Linear")
      (`GameplayStatics.PlaySound2D` "/Game/JadeCiderquist/Sound/Kraken_Roar.Kraken_Roar" 1.0 1.0 0.0 null null))))

(event `self.HengSao_Bottom.OnComponentEndOverlap`
  (params (OverlappedComponent :type "PrimitiveComponent Object Reference") (OtherActor :type "Actor Object Reference") (OtherComp :type "PrimitiveComponent Object Reference") (OtherBodyIndex :type Integer))
  ;[1 1 1] 底部横扫重叠
  (cast `/Game/AFCore/Examples/Pawns/VR/BP_Pawn_VR_Char_Example_HandsOn` OtherActor)
  (set `self.Bottom_Attack` false)
  (`|ExecutionSequence`
    (:`then_0`
      (goto _label_7 :!via `Close`))
    (:`then_1`
      (goto _label_8 :!via `Close`))
    (:`then_2`
      ;[1 1 1] 攻击范围文字提示
      (bind _outactors (`GameplayStatics.GetAllActorsOfClass` "/Game/AFCore/Examples/Pawns/VR/BP_Pawn_VR_Char_Example_HandsOn.BP_Pawn_VR_Char_Example_HandsOn_C"))
      (bind _output (`|GetArrayItem` _outactors))
      (bind _wbp_bossredup (`/Game/AFCore/Examples/Pawns/VR/BP_Pawn_VR_Char_Example_HandsOn.WBP_BOSSredup` _output))
      (if (`SceneComponent.IsVisible` _wbp_bossredup)
        (`SceneComponent.SetVisibility` _wbp_bossredup false false)
        (bind _wbp_bossgreen (`/Game/AFCore/Examples/Pawns/VR/BP_Pawn_VR_Char_Example_HandsOn.WBP_BOSSgreen` _output))
        (`SceneComponent.SetVisibility` _wbp_bossgreen true false)
        (`KismetSystemLibrary.Delay` 2.0)
        (`SceneComponent.SetVisibility` _wbp_bossgreen false false)))))

(event `self.Attack_FanWei.OnComponentBeginOverlap`
  (params (OverlappedComponent :type "PrimitiveComponent Object Reference") (OtherActor :type "Actor Object Reference") (OtherComp :type "PrimitiveComponent Object Reference") (OtherBodyIndex :type Integer) (bFromSweep :type Boolean) (SweepResult :type "HitResult Structure (by ref)"))
  ;[1 1 1] 角色进入范围开始近战攻击
  (cast `/Game/AFCore/Examples/Pawns/VR/BP_Pawn_VR_Char_Example_HandsOn` OtherActor)
  (`|ExecutionSequence`
    (:`then_0`
      (set `self.if_CloseAttack` true)
      (goto _label_11 :!via `Close`))
    (:`then_1`
      ;[1 1 1] 播放Boss BGM
      (`/Engine/EditorBlueprintResources/StandardMacros.DoOnce` false
        (:`Completed`
          (`AudioComponent.FadeIn` (`self.BGM`) 1.0 1.0 0.0 "Linear"))))))

(event `self.Mouse_Sphere.OnComponentBeginOverlap`
  (params (OverlappedComponent :type "PrimitiveComponent Object Reference") (OtherActor :type "Actor Object Reference") (OtherComp :type "PrimitiveComponent Object Reference") (OtherBodyIndex :type Integer) (bFromSweep :type Boolean) (SweepResult :type "HitResult Structure (by ref)"))
  (bind _comp_widget (`self.Comp_Widget`))
  (bind (_returnvalue_x _returnvalue_y) (`KismetMathLibrary.BreakVector2D` (`WidgetComponent.GetDrawSize` _comp_widget)))
  ;[1 1 1] 命中嘴巴多扣一次
  (bind _asprojectile (cast `/Game/JadeCiderquist/Gun/Blueprints/Projectile` OtherActor))
  (if (not (`self.if_Death`))
    (`ActorComponent.Activate` (`/Game/JadeCiderquist/Gun/Blueprints/Projectile.VFX_GrenadeEXP_air` _asprojectile) false)
    (`GameplayStatics.PlaySound2D` "/Game/JadeCiderquist/Sound/Gun_hit.Gun_hit" 1.0 1.0 0.0 null null)
    ;[1 1 1] 伤害
    (bind _output_get (set `self.Health` (- (stale _output_get) (/ (`/Game/JadeCiderquist/Gun/Blueprints/Projectile.Harm` _asprojectile) 60.0))))
    (`WidgetComponent.SetDrawSize` _comp_widget (`KismetMathLibrary.MakeVector2D` (* 3000.0 (`self.Health`)) _returnvalue_y))
    (goto _label_13)))

(event `self.AttackFar_Sphere.OnComponentBeginOverlap`
  (params (OverlappedComponent :type "PrimitiveComponent Object Reference") (OtherActor :type "Actor Object Reference") (OtherComp :type "PrimitiveComponent Object Reference") (OtherBodyIndex :type Integer) (bFromSweep :type Boolean) (SweepResult :type "HitResult Structure (by ref)"))
  ;[1 1 1] 喷墨水
  (bind _asbp_pawn_vr_char_example_hands_on (cast `/Game/AFCore/Examples/Pawns/VR/BP_Pawn_VR_Char_Example_HandsOn` OtherActor))
  (set `/Game/AFCore/Examples/Pawns/VR/BP_Pawn_VR_Char_Example_HandsOn.PlayerRe_Location` (`self.Boss_PlayerRe_Location`) _asbp_pawn_vr_char_example_hands_on)
  (set `/Game/AFCore/Examples/Pawns/VR/BP_Pawn_VR_Char_Example_HandsOn.Speed_Scale` 5.0 _asbp_pawn_vr_char_example_hands_on)
  (set `self.if_FarAttack` true)
  (goto _label_12 :!via `Open`))

(event `self.AttackFar_Sphere.OnComponentEndOverlap`
  (params (OverlappedComponent :type "PrimitiveComponent Object Reference") (OtherActor :type "Actor Object Reference") (OtherComp :type "PrimitiveComponent Object Reference") (OtherBodyIndex :type Integer))
  ;[1 1 1] 喷墨水
  (bind _asbp_pawn_vr_char_example_hands_on (cast `/Game/AFCore/Examples/Pawns/VR/BP_Pawn_VR_Char_Example_HandsOn` OtherActor))
  (set `/Game/AFCore/Examples/Pawns/VR/BP_Pawn_VR_Char_Example_HandsOn.Speed_Scale` 1.5 _asbp_pawn_vr_char_example_hands_on)
  (set `self.if_FarAttack` false)
  (goto _label_12 :!via `Close`))

(event `self.HengSao_Up.OnComponentBeginOverlap`
  (params (OverlappedComponent :type "PrimitiveComponent Object Reference") (OtherActor :type "Actor Object Reference") (OtherComp :type "PrimitiveComponent Object Reference") (OtherBodyIndex :type Integer) (bFromSweep :type Boolean) (SweepResult :type "HitResult Structure (by ref)"))
  ;[1 1 1] 顶部横扫重叠
  (cast `/Game/AFCore/Examples/Pawns/VR/BP_Pawn_VR_Char_Example_HandsOn` OtherActor)
  (set `self.Top_Attack` true)
  (set `self.if_CloseAttack` true)
  ;;[0 0.2974 1] 顶部横扫攻击
  (set `self.Int_At` 2)
  ;[1 1 1] 攻击范围文字提示
  (`|ExecutionSequence`
    (:`then_0`
      (goto _label_9 :!via `Open`))
    (:`then_1`
      (goto _label_10 :!via `Open`))))

(event `self.HengSao_Up.OnComponentEndOverlap`
  (params (OverlappedComponent :type "PrimitiveComponent Object Reference") (OtherActor :type "Actor Object Reference") (OtherComp :type "PrimitiveComponent Object Reference") (OtherBodyIndex :type Integer))
  ;[1 1 1] 顶部横扫重叠
  (cast `/Game/AFCore/Examples/Pawns/VR/BP_Pawn_VR_Char_Example_HandsOn` OtherActor)
  (set `self.Top_Attack` false)
  (`|ExecutionSequence`
    (:`then_0`
      (goto _label_9 :!via `Close`))
    (:`then_1`
      (goto _label_10 :!via `Close`))
    (:`then_2`
      ;[1 1 1] 攻击范围文字提示
      (bind _outactors (`GameplayStatics.GetAllActorsOfClass` "/Game/AFCore/Examples/Pawns/VR/BP_Pawn_VR_Char_Example_HandsOn.BP_Pawn_VR_Char_Example_HandsOn_C"))
      (bind _output (`|GetArrayItem` _outactors))
      (bind _wbp_bossreddown (`/Game/AFCore/Examples/Pawns/VR/BP_Pawn_VR_Char_Example_HandsOn.WBP_BOSSreddown` _output))
      (if (`SceneComponent.IsVisible` _wbp_bossreddown)
        (`SceneComponent.SetVisibility` _wbp_bossreddown false false)
        (bind _wbp_bossgreen (`/Game/AFCore/Examples/Pawns/VR/BP_Pawn_VR_Char_Example_HandsOn.WBP_BOSSgreen` _output))
        (`SceneComponent.SetVisibility` _wbp_bossgreen true false)
        (`KismetSystemLibrary.Delay` 2.0)
        (`SceneComponent.SetVisibility` _wbp_bossgreen false false)))))

(fn `UserConstructionScript`)