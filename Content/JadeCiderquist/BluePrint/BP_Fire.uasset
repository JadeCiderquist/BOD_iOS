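; BP_Fire is a collectible flame in a VR scene, picked up when a projectile hits its sphere.
; A hit plays left-hand haptics and sound, and, within the pawn's FireCount limit, registers the flame on the pawn and removes the sphere.
; A timeline pulls it toward the left-side arrow while dimming its light and shrinking its Niagara effect.
; Tick then pins it to its indexed pawn arrow, looking up the pawn every frame.
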(event `self.ReceiveTick`
  (params (DeltaSeconds :type "Float (single-precision)"))
  (bind _outactors (`GameplayStatics.GetAllActorsOfClass` "/Game/AFCore/Examples/Pawns/VR/BP_Pawn_VR_Char_Example_HandsOn.BP_Pawn_VR_Char_Example_HandsOn_C"))
  ;[1 1 1] 获取三个点的坐标并设置位置
  (if (`self.Get`)
    (switch `int` (`self.Count`)
      (:`0`
        (bind _output (`|GetArrayItem` (`/Game/AFCore/Examples/Pawns/VR/BP_Pawn_VR_Char_Example_HandsOn.Arrow_Count` (`|GetArrayItem` _outactors)) (`self.Count`)))
        (`self.K2_SetActorLocation` (`SceneComponent.K2_GetComponentLocation` _output)))
      (:`1`
        (`self.K2_SetActorLocation` (`SceneComponent.K2_GetComponentLocation` _output)))
      (:`2`
        (`self.K2_SetActorLocation` (`SceneComponent.K2_GetComponentLocation` _output)))
      (:`3`
        (`self.K2_SetActorLocation` (`SceneComponent.K2_GetComponentLocation` _output)))
      (:`4`
        (`self.K2_SetActorLocation` (`SceneComponent.K2_GetComponentLocation` _output)))
      (:`5`
        (`self.K2_SetActorLocation` (`SceneComponent.K2_GetComponentLocation` _output))))))

(event `self.Sphere.OnComponentBeginOverlap`
  (params (OverlappedComponent :type "PrimitiveComponent Object Reference") (OtherActor :type "Actor Object Reference") (OtherComp :type "PrimitiveComponent Object Reference") (OtherBodyIndex :type Integer) (bFromSweep :type Boolean) (SweepResult :type "HitResult Structure (by ref)"))
  (bind _pointlight (`self.PointLight`))
  (bind _ns_rocketexhaust_blue (`self.NS_RocketExhaust_Blue`))
  ;[1 1 1] 触碰火焰后手柄震动
  (cast `/Game/JadeCiderquist/Gun/Blueprints/Projectile` OtherActor)
  (`PlayerController.PlayHapticEffect` (`GameplayStatics.GetPlayerController` 0) "/Game/JadeCiderquist/Gun/Haptics/FireHapticEffect.FireHapticEffect" "Left" 1.0 false)
  (`GameplayStatics.PlaySound2D` "/Game/JadeCiderquist/Sound/MainBuilding_lightup.MainBuilding_lightup" 1.0 1.0 0.0 null null)
  (`SceneComponent.SetVisibility` (`self.SM_YinDaoQi2`) false false)
  (bind _output (`|GetArrayItem` (stale `self.ReceiveTick` _outactors)))
  ;[0 0 0] 在火焰<=5时可以继续获取火焰
  (if (<= (`/Game/AFCore/Examples/Pawns/VR/BP_Pawn_VR_Char_Example_HandsOn.Fire_Count` _output) 5)
    (bind _outactors (`GameplayStatics.GetAllActorsOfClass` "/Game/AFCore/Examples/Pawns/VR/BP_Pawn_VR_Char_Example_HandsOn.BP_Pawn_VR_Char_Example_HandsOn_C"))
    (bind _outactors_2 (`GameplayStatics.GetAllActorsOfClass` "/Game/AFCore/Examples/Pawns/VR/BP_Pawn_VR_Char_Example_HandsOn.BP_Pawn_VR_Char_Example_HandsOn_C"))
    (`KismetArrayLibrary.Array_Add` (`/Game/AFCore/Examples/Pawns/VR/BP_Pawn_VR_Char_Example_HandsOn.BP_Fire` (`|GetArrayItem` _outactors_2)) self)
    ;[1 1 1] 删除碰撞体避免重复碰撞
    (bind _output_get (set `/Game/AFCore/Examples/Pawns/VR/BP_Pawn_VR_Char_Example_HandsOn.Fire_Count` (+ (stale _output_get) 1) _output))
    (`ActorComponent.K2_DestroyComponent` (`self.Sphere`))
    (`/Engine/EditorBlueprintResources/StandardMacros.DoOnce` false
      (:`Completed`
        (set `self.Count` (- _output_get 1))
        (bind (_direction `_新建轨道_0`) (`Timeline|时间轴_0` :`NewTime` 0.0)
          (:`Update`
            (`self.K2_SetActorLocation` (`KismetMathLibrary.VLerp` (`self.K2_GetActorLocation`) (`SceneComponent.K2_GetComponentLocation` (`/Game/AFCore/Blueprints/Pawn/VR/BP_Pawn_VR.LeftSideArrow` (`|GetArrayItem` _outactors))) `_新建轨道_0`))
            (`LightComponent.SetIntensity` _pointlight (`KismetMathLibrary.Lerp` (`self.强度`) 0.0 `_新建轨道_0`))
            ;[1 1 1] 粒子缩小效果
            (`NiagaraComponent.SetVariableFloat` _ns_rocketexhaust_blue "Drag" 100.0)
            (`NiagaraComponent.SetVariableFloat` _ns_rocketexhaust_blue "Scale" (`KismetMathLibrary.Lerp` 2.0 0.15 `_新建轨道_0`))
            (`NiagaraComponent.SetVariableFloat` _ns_rocketexhaust_blue "HeatHaze_SpawnRate" 0.0)
            (`NiagaraComponent.SetVariableVec3` _ns_rocketexhaust_blue "Thrusters_AttractionPoint" (0.0 0.0 0.0))
            (`NiagaraComponent.SetVariableFloat` _ns_rocketexhaust_blue "Thrusters_SpawnRate" 50.0)
            (`SceneComponent.SetRelativeScale3D` _ns_rocketexhaust_blue (`KismetMathLibrary.Conv_DoubleToVector` (`KismetMathLibrary.Lerp` 1.0 0.2 `_新建轨道_0`))))
          (:`Finished`
            (`SceneComponent.SetVisibility` _pointlight false false)
            (set `self.Get` true)))))))

(fn `UserConstructionScript`
  (bind _pointlight (`self.PointLight`))
  (`LightComponent.SetIntensity` _pointlight (`self.强度`))
  (`PointLightComponent.SetSourceRadius` _pointlight (`self.源半径`))
  (`LocalLightComponent.SetAttenuationRadius` _pointlight (`self.衰减半径`))
  (`SceneComponent.SetVisibility` (`self.SM_YinDaoQi2`) (`self.引导`) false))