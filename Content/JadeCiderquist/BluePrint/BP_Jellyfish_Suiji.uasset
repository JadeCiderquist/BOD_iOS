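; Spawner actor that populates the area around itself with BP_Jellyfish instances, one per second from BeginPlay.
; A delayed loop spawns each at zero scale at a random radius-based offset, with half the spread vertically.
; Each gets random Speed and Lenth values and a fixed light intensity, while its random target scale is stored in JelScale.
; One shared timeline restarts on every spawn to grow the newest jellyfish to that scale.
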(event `self.ReceiveBeginPlay`
  (bind _radius_max (`self.Radius_Max`))
  (bind _radius_min (`self.Radius_Min`))
  (bind _returnvalue (`KismetMathLibrary.RandomFloatInRange` _radius_min _radius_max))
  (bind _returnvalue_2 (`KismetMathLibrary.RandomFloatInRange` _radius_min _radius_max))
  (bind _returnvalue_3 (`KismetMathLibrary.RandomFloatInRange` _radius_min _radius_max))
  (`/Game/AFCore/Libraries/MLib_Actor_Macros.ForLoopWithDelay` 0 (`self.Count`) 1.0
    (:`LoopBody`
      (bind _returnvalue_4 (`|SpawnActorFromClass` "/Game/JadeCiderquist/BluePrint/BP_Jellyfish.BP_Jellyfish_C" (`KismetMathLibrary.MakeTransform` (+ (`self.K2_GetActorLocation`) (`KismetMathLibrary.MakeVector` (`KismetMathLibrary.RandomFloatInRange` (* _returnvalue -1.0) _returnvalue) (`KismetMathLibrary.RandomFloatInRange` (* _returnvalue_2 -1.0) _returnvalue_2) (/ (`KismetMathLibrary.RandomFloatInRange` (* _returnvalue_3 -1.0) _returnvalue_3) 2.0))) (struct) (0.0 0.0 0.0)) "Undefined" "MultiplyWithRoot" null null))
      (bind _returnvalue_5 (`KismetArrayLibrary.Array_Add` (`self.Jel_Scale`) (`KismetMathLibrary.Conv_DoubleToVector` (`KismetMathLibrary.RandomFloatInRange` 0.01 0.5))))
      (set `/Game/JadeCiderquist/BluePrint/BP_Jellyfish.Speed` (`KismetMathLibrary.RandomFloatInRange` 0.1 2.0) _returnvalue_4)
      (set `/Game/JadeCiderquist/BluePrint/BP_Jellyfish.Lenth` (`KismetMathLibrary.RandomFloatInRange` 1000.0 5000.0) _returnvalue_4)
      (`LightComponent.SetIntensity` (`/Game/JadeCiderquist/BluePrint/BP_Jellyfish.PointLight` _returnvalue_4) 500.0)
      (bind (_direction `_新建轨道_0`) (`Timeline|时间轴` :!via `PlayFromStart`)
        (:`Update`
          (`self.SetActorRelativeScale3D` _returnvalue_4 (`KismetMathLibrary.VLerp` (0.0 0.0 0.0) (`|GetArrayItem` (`self.Jel_Scale`) _returnvalue_5) `_新建轨道_0`)))))))

(fn `UserConstructionScript`)