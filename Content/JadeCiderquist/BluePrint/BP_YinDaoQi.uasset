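; BP_YinDaoQi is a spline-driven placement actor that repeats a chosen mesh at regular intervals along its path.
; The construction script divides the spline length by LocationLenth and adds a spline mesh component at each step.
; Each component is positioned and rotated from the spline's local location and direction, with 90-degree roll and yaw offsets, without bending.
; The material override is disconnected, and the event graph is empty.
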(fn `UserConstructionScript`
  (bind _location_lenth (`self.Location_Lenth`))
  (bind _spline (`self.Spline`))
  (bind _start_location (`self.Start_Location`))
  (bind _returnvalue (`SplineComponent.GetDirectionAtDistanceAlongSpline` _spline _start_location "Local"))
  (bind (_returnvalue_roll _returnvalue_pitch) (`KismetMathLibrary.BreakRotator` (`KismetMathLibrary.MakeRotFromZ` _returnvalue)))
  (for _ (range (+ (`KismetMathLibrary.FCeil` (/ (`SplineComponent.GetSplineLength` _spline) _location_lenth)) 1))
    (bind _returnvalue_2 (`AddComponent|NODE_AddSplineMeshComponent-0`))
    (`StaticMeshComponent.SetStaticMesh` _returnvalue_2 (`self.Mesh`))
    (`SceneComponent.K2_SetRelativeLocation` _returnvalue_2 (0.0 0.0 0.0) false false)
    (set `self.Start_Location` (+ _location_lenth _start_location))
    (`SceneComponent.K2_SetRelativeLocation` _returnvalue_2 (`SplineComponent.GetLocationAtDistanceAlongSpline` _spline _start_location "Local") false false)
    (`SceneComponent.K2_SetRelativeRotation` _returnvalue_2 (`KismetMathLibrary.MakeRotator` (+ _returnvalue_roll 90.0) _returnvalue_pitch (+ (.yaw (`KismetMathLibrary.MakeRotFromX` _returnvalue)) 90.0)) false false)
    (`self.K2_AttachToComponent` _returnvalue_2 "None" "KeepRelative" "KeepRelative" "KeepRelative")))