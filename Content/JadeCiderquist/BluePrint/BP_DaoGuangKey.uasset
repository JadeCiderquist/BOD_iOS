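; BP_DaoGuangKey is a grabbable VR key actor with a zone that affects the player's shark detection and speed.
; Pickup hides the SMYinDaoQi mesh, then calls GrabReleased on its grab component after a short delay.
; Entering Shark_Sphere collapses the first VR pawn's shark detection sphere and lowers its SpeedScale; leaving sets both to fixed higher values.
; The default events and construction script are empty.
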(event `self.Comp_Grab.Grab_ActorPickedUp`
  (params (GrabbingPawn :type "/Game/AFCore/Blueprints/Pawn/BP_Pawn_Base Object Reference") (GrabbingActor :type "Actor Object Reference"))
  (`SceneComponent.SetVisibility` (`self.SM_YinDaoQi`) false false)
  (`KismetSystemLibrary.Delay` 1.0)
  (`/Game/AFCore/Blueprints/Components/Interaction/Comp_Grab.GrabReleased` (`self.Comp_Grab`) self))

(event `self.Shark_Sphere.OnComponentBeginOverlap`
  (params (OverlappedComponent :type "PrimitiveComponent Object Reference") (OtherActor :type "Actor Object Reference") (OtherComp :type "PrimitiveComponent Object Reference") (OtherBodyIndex :type Integer) (bFromSweep :type Boolean) (SweepResult :type "HitResult Structure (by ref)"))
  ;[1 1 1] 设置角色鲨鱼检测球体半径
  (cast `/Game/AFCore/Examples/Pawns/VR/BP_Pawn_VR_Char_Example_HandsOn` OtherActor)
  (bind _outactors (`GameplayStatics.GetAllActorsOfClass` "/Game/AFCore/Examples/Pawns/VR/BP_Pawn_VR_Char_Example_HandsOn.BP_Pawn_VR_Char_Example_HandsOn_C"))
  (bind _output (`|GetArrayItem` _outactors))
  (`SphereComponent.SetSphereRadius` (`/Game/AFCore/Examples/Pawns/VR/BP_Pawn_VR_Char_Example_HandsOn.Sharke_Sphere` _output) 0.0 true)
  (set `/Game/AFCore/Examples/Pawns/VR/BP_Pawn_VR_Char_Example_HandsOn.Speed_Scale` 0.5 _output))

(event `self.Shark_Sphere.OnComponentEndOverlap`
  (params (OverlappedComponent :type "PrimitiveComponent Object Reference") (OtherActor :type "Actor Object Reference") (OtherComp :type "PrimitiveComponent Object Reference") (OtherBodyIndex :type Integer))
  ;[1 1 1] 设置角色鲨鱼检测球体半径
  (cast `/Game/AFCore/Examples/Pawns/VR/BP_Pawn_VR_Char_Example_HandsOn` OtherActor)
  (bind _outactors (`GameplayStatics.GetAllActorsOfClass` "/Game/AFCore/Examples/Pawns/VR/BP_Pawn_VR_Char_Example_HandsOn.BP_Pawn_VR_Char_Example_HandsOn_C"))
  (bind _output (`|GetArrayItem` _outactors))
  (`SphereComponent.SetSphereRadius` (`/Game/AFCore/Examples/Pawns/VR/BP_Pawn_VR_Char_Example_HandsOn.Sharke_Sphere` _output) 180.0 true)
  (set `/Game/AFCore/Examples/Pawns/VR/BP_Pawn_VR_Char_Example_HandsOn.Speed_Scale` 1.5 _output))

(fn `UserConstructionScript`)