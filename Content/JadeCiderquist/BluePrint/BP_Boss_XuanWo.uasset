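; Boss vortex actor that acts as a transition trigger for the VR player, tinting its vortex effect from a Color variable at BeginPlay.
; Sphere overlap locks player movement and fades to black before restoring movement.
; IfAllGame then either teleports the player to the third light tower, fades in and hides door guides, or destroys the Pistol and opens the Final level.
; An alpha fade-in timeline for the vortex is unconnected.
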(event `self.ReceiveBeginPlay`
  (`NiagaraComponent.SetVariableLinearColor` (`self.NS_Vortex_Boss`) "XW_Color" (`self.Color`)))

(event `self.Sphere.OnComponentBeginOverlap`
  (params (OverlappedComponent :type "PrimitiveComponent Object Reference") (OtherActor :type "Actor Object Reference") (OtherComp :type "PrimitiveComponent Object Reference") (OtherBodyIndex :type Integer) (bFromSweep :type Boolean) (SweepResult :type "HitResult Structure (by ref)"))
  (bind _asbp_pawn_vr_char_example_hands_on (cast `/Game/AFCore/Examples/Pawns/VR/BP_Pawn_VR_Char_Example_HandsOn` OtherActor))
  (set `/Game/AFCore/Examples/Pawns/VR/BP_Pawn_VR_Char_Example_HandsOn.if_Move` false _asbp_pawn_vr_char_example_hands_on)
  (`PlayerCameraManager.StartCameraFade` :`self` (`GameplayStatics.GetPlayerCameraManager` 0) :`ToAlpha` 1.0 :`Duration` 2.0)
  (`KismetSystemLibrary.Delay` 2.0)
  (bind _outactors (`GameplayStatics.GetAllActorsOfClass` "/Game/AFCore/Examples/Pawns/VR/BP_Pawn_VR_Char_Example_HandsOn.BP_Pawn_VR_Char_Example_HandsOn_C"))
  (set `/Game/AFCore/Examples/Pawns/VR/BP_Pawn_VR_Char_Example_HandsOn.if_Move` true (`|GetArrayItem` _outactors))
  (if (`self.if_AllGame`)
    ;[1 1 1] 瞬移至第三座导光塔
    (bind _outactors_2 (`GameplayStatics.GetAllActorsOfClass` "/Game/AFCore/Examples/Pawns/VR/BP_Pawn_VR_Char_Example_HandsOn.BP_Pawn_VR_Char_Example_HandsOn_C"))
    (`self.K2_SetActorLocation` (`|GetArrayItem` _outactors_2) (`self.New Location`) false false)
    ;[1 1 1] 黑场变亮
    (`PlayerCameraManager.StartCameraFade` :`self` (`GameplayStatics.GetPlayerCameraManager` 0) :`FromAlpha` 1.0 :`Duration` 2.0)
    ;[1 1 1] 关闭门引导
    (bind _outactors_3 (`GameplayStatics.GetAllActorsOfClass` "/Game/JadeCiderquist/BluePrint/BP_Door_Col.BP_Door_Col_C"))
    (`SceneComponent.SetVisibility` (`/Game/JadeCiderquist/BluePrint/BP_Door_Col.SM_YinDaoQi` (`|GetArrayItem` _outactors_3)) false false)
    (`SceneComponent.SetVisibility` (`/Game/JadeCiderquist/BluePrint/BP_Door_Col.SM_YinDaoQi` (`|GetArrayItem` _outactors_3 1)) false false)
    (else
      (bind _outactors_4 (`GameplayStatics.GetAllActorsOfClass` "/Game/JadeCiderquist/Gun/Blueprints/Pistol.Pistol_C"))
      (`self.K2_DestroyActor` (`|GetArrayItem` _outactors_4))
      (`GameplayStatics.OpenLevelBySoftObjectPtr` "/Game/Final.Final"))))

(fn `UserConstructionScript`)