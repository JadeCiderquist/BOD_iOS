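; Hand-scanner interactable that activates a light-guide tower when the VR player has at least three collected fires.
; Overlapping its sphere shows the prompt and opens a gate for interaction, which consumes fires and updates the checkpoint.
; HandCount selects the tagged tower and stage-specific guidance and spotlights.
; Timelines animate glowing lines and the beam, then signal BP_MainBuilding; an incomplete second tower holds that signal until ComTA fires.
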(event `self.ReceiveBeginPlay`
  (bind _spot_light (`self.Spot_Light`))
  (bind _returnvalue (`|CreateWidget` "/Game/JadeCiderquist/Widget/Button/E_JiHuo.E_JiHuo_C" (`GameplayStatics.GetPlayerController` 0)))
  (set `self.W_JiHuo` _returnvalue)
  (bind _returnvalue_2 (`PrimitiveComponent.CreateDynamicMaterialInstance` (`self.SM_Handscanner`) 1 "/Game/WengZhiBo/Material/M_Fire.M_Fire" "None"))
  (set `self.DynMaterial` _returnvalue_2)
  ;[1 1 1] 开始运行灯光关闭
  (bind (_array_element _array_index) (`/Game/AFCore/Libraries/MLib_Actor_Macros.ForEachLoopWithDelay` _spot_light)
    (:`LoopBody`
      (`LightComponent.SetIntensity` (`Light.LightComponent` (`|GetArrayItem` _spot_light _array_index)) 0.0))))

(event `self.Comp_Latch.Latch_ActorGotLatched`
  (params (LatchingPawn :type "/Game/AFCore/Blueprints/Pawn/BP_Pawn_Base Object Reference") (LatchingActor :type "Actor Object Reference"))
  (cast `/Game/AFCore/Blueprints/VR/MotionComponents/BP_MComp` LatchingActor))

(event `/Game/JadeCiderquist/BluePrint/BI_OpenBuilding.Open/Interacte`
  (bind _hand_count (`self.Hand_Count`))
  (bind _hand_count_2 (`self.Hand_Count`))
  (bind _spot_light (`self.Spot_Light`))
  (`/Engine/EditorBlueprintResources/StandardMacros.Gate` true :!label _label
    (:`Exit`
      (`Widget.RemoveFromParent` (`self.W_JiHuo`))
      (`SceneComponent.SetVisibility` (`self.SM_YinDaoQi`) false false)
      (`MaterialInstanceDynamic.SetVectorParameterValue` (`self.DynMaterial`) "color" (struct :`G` 0.794128 :`B` 2.0 :`A` 1.0))
      (bind _outactors (`GameplayStatics.GetAllActorsOfClass` "/Game/AFCore/Examples/Pawns/VR/BP_Pawn_VR_Char_Example_HandsOn.BP_Pawn_VR_Char_Example_HandsOn_C"))
      (bind _output (`|GetArrayItem` _outactors))
      (if (>= (`/Game/AFCore/Examples/Pawns/VR/BP_Pawn_VR_Char_Example_HandsOn.Fire_Count` _output) 3)
        ;[1 1 1] 成功
        (`SceneComponent.SetVisibility` (`self.Decal`) false false)
        (switch `ETimelineDirection` "Forward"
          (:`Forward`
            (`MaterialInstanceDynamic.SetVectorParameterValue` (`self.DynMaterial`) "color" (struct :`G` 5.722922 :`B` 15.0 :`A` 1.0))
            (if (== _hand_count_2 0)
              ;[1 1 1] 只能点一次塔
              (`/Engine/EditorBlueprintResources/StandardMacros.DoOnce` false
                (:`Completed`
                  ;[1 1 1] 主建筑动画
                  (bind _outactors_2 (`GameplayStatics.GetAllActorsOfClass` "/Game/JadeCiderquist/BluePrint/BP_MainBuilding.BP_MainBuilding_C"))
                  (bind _output_2 (`|GetArrayItem` _outactors_2))
                  (`SkeletalMeshComponent.Play` (`/Game/JadeCiderquist/BluePrint/BP_MainBuilding.ANI_landmark` _output_2) false)
                  (`AudioComponent.Play` (`/Game/JadeCiderquist/BluePrint/BP_MainBuilding.Audio` _output_2) 0.0)
                  ;[1 1 1] 第二座塔红色引导球
                  (bind _outactors_3 (`GameplayStatics.GetAllActorsOfClassWithTag` "/Game/JadeCiderquist/BluePrint/BP_DaoGuangTa.BP_DaoGuangTa_C" "TA1"))
                  (bind _output_3 (`|GetArrayItem` _outactors_3))
                  (`self.SetActorHiddenInGame` _output_3 false)
                  (`SceneComponent.SetVisibility` (`/Game/JadeCiderquist/BluePrint/BP_DaoGuangTa.YinDao_Sphere` _output_3) true false)
                  ;[1 1 1] 拉杆引导可视
                  (bind _outactors_4 (`GameplayStatics.GetAllActorsOfClass` "/Game/AFCore/Examples/Blueprints/HandsOn/BP_Lever_WidgetExample.BP_Lever_WidgetExample_C"))
                  (`SceneComponent.SetVisibility` (`/Game/AFCore/Examples/Blueprints/HandsOn/BP_Lever_WidgetExample.SM_YinDaoQi` (`|GetArrayItem` _outactors_4)) true false)
                  (`|ExecutionSequence`
                    (:`then_0`
                      ;[1 1 1] 前往第二座导光塔引导
                      (`KismetSystemLibrary.Delay` 8.0)
                      (bind _outactors_5 (`GameplayStatics.GetAllActorsOfClass` "/Game/AFCore/Examples/Pawns/VR/BP_Pawn_VR_Char_Example_HandsOn.BP_Pawn_VR_Char_Example_HandsOn_C"))
                      (bind _output_4 (`|GetArrayItem` _outactors_5))
                      (bind _wbp_2tower (`/Game/AFCore/Examples/Pawns/VR/BP_Pawn_VR_Char_Example_HandsOn.WBP_2Tower` _output_4))
                      (`SceneComponent.SetVisibility` _wbp_2tower true false)
                      (`KismetSystemLibrary.Delay` 8.0)
                      (`SceneComponent.SetVisibility` _wbp_2tower false false)
                      (`KismetSystemLibrary.Delay` 1.0)
                      (bind _wbp_gamepoint (`/Game/AFCore/Examples/Pawns/VR/BP_Pawn_VR_Char_Example_HandsOn.WBP_GamePoint` _output_4))
                      (`SceneComponent.SetVisibility` _wbp_gamepoint true false)
                      (`KismetSystemLibrary.Delay` 8.0)
                      (`SceneComponent.SetVisibility` _wbp_gamepoint false false))
                    (:`then_1`
                      ;[1 1 1] 删除3个火焰
                      (for _ (range 3) :!label _label_2
                        (bind _outactors_6 (`GameplayStatics.GetAllActorsOfClass` "/Game/AFCore/Examples/Pawns/VR/BP_Pawn_VR_Char_Example_HandsOn.BP_Pawn_VR_Char_Example_HandsOn_C"))
                        (bind _bp_fire (`/Game/AFCore/Examples/Pawns/VR/BP_Pawn_VR_Char_Example_HandsOn.BP_Fire` (`|GetArrayItem` _outactors_6)))
                        (bind _output_5 (`|GetArrayItem` _bp_fire (- (`KismetArrayLibrary.Array_Length` _bp_fire) 1)))
                        (`self.K2_DestroyActor` _output_5)
                        (`KismetArrayLibrary.Array_RemoveItem` _bp_fire _output_5)
                        ;[1 1 1] 线条发光
                        (bind _outactors_7 (`GameplayStatics.GetAllActorsOfClassWithTag` "/Game/JadeCiderquist/BluePrint/BP_DaoGuangTa.BP_DaoGuangTa_C" (`|GetArrayItem` (`self.Tag`) (`self.Hand_Count`))))
                        (bind _output_6 (`|GetArrayItem` _outactors_7))
                        (bind _returnvalue (`PrimitiveComponent.CreateDynamicMaterialInstance` (`/Game/JadeCiderquist/BluePrint/BP_DaoGuangTa.M_LightC` _output_6) 0 "/Game/JadeCiderquist/Material/Light_Ta_Red.Light_Ta_Red" "None"))
                        (`MaterialInstanceDynamic.SetScalarParameterValue` _returnvalue "Alpha" 0.0)
                        (bind _returnvalue_2 (`PrimitiveComponent.CreateDynamicMaterialInstance` (`/Game/JadeCiderquist/BluePrint/BP_DaoGuangTa.MechanismA_Mechanism05_F` _output_6) 0 "/Game/JadeCiderquist/Material/M_Line_Color.M_Line_Color" "None"))
                        (bind _returnvalue_3 (`PrimitiveComponent.CreateDynamicMaterialInstance` (`/Game/JadeCiderquist/BluePrint/BP_DaoGuangTa.Mechanism_Add` _output_6) 0 "/Game/JadeCiderquist/Material/M_Line_Color.M_Line_Color" "None"))
                        (bind (_direction `_新建轨道_0`) (`Timeline|时间轴_0`)
                          (:`Update`
                            (`MaterialInstanceDynamic.SetScalarParameterValue` _returnvalue_2 "Pos" (`KismetMathLibrary.Lerp` 0.0 3.0 `_新建轨道_0`))
                            (`MaterialInstanceDynamic.SetScalarParameterValue` _returnvalue_3 "Pos" (`KismetMathLibrary.Lerp` 0.0 3.0 `_新建轨道_0`))
                            (`/Engine/EditorBlueprintResources/StandardMacros.DoOnce` false
                              (:`Completed`
                                (`KismetSystemLibrary.Delay` 1.0)
                                (bind _audio (`/Game/JadeCiderquist/BluePrint/BP_DaoGuangTa.Audio` _output_6))
                                (`AudioComponent.Play` _audio 0.0))))
                          (:`Finished`
                            (`AudioComponent.Stop` _audio)
                            ;[1 1 1] 导光塔存档点
                            (bind _outactors_8 (`GameplayStatics.GetAllActorsOfClass` "/Game/AFCore/Examples/Pawns/VR/BP_Pawn_VR_Char_Example_HandsOn.BP_Pawn_VR_Char_Example_HandsOn_C"))
                            (bind _output_7 (`|GetArrayItem` _outactors_8))
                            (set `/Game/AFCore/Examples/Pawns/VR/BP_Pawn_VR_Char_Example_HandsOn.PlayerRe_Location` (`self.K2_GetActorLocation` _output_7) _output_7)
                            ;[1 1 1] 光束发射
                            (bind _outactors_9 (`GameplayStatics.GetAllActorsOfClassWithTag` "/Game/JadeCiderquist/BluePrint/BP_GuangShu.BP_GuangShu_C" (`|GetArrayItem` (`self.Tag`) (`self.Hand_Count`))))
                            (bind _output_8 (`|GetArrayItem` _outactors_9))
                            (`ActorComponent.Activate` (`/Game/JadeCiderquist/BluePrint/BP_GuangShu.NS_LightTa` _output_8) false)
                            (bind _returnvalue_4 (`PrimitiveComponent.CreateDynamicMaterialInstance` (`/Game/JadeCiderquist/BluePrint/BP_GuangShu.M_LightC` _output_8) 0 "/Game/JadeCiderquist/Material/Light_Ta_Inst.Light_Ta_Inst" "None"))
                            (`MaterialInstanceDynamic.SetScalarParameterValue` _returnvalue_4 "Alpha" 5.0)
                            (`AudioComponent.Play` (`/Game/JadeCiderquist/BluePrint/BP_GuangShu.Audio` _output_8) 0.0)
                            (bind (_direction_2 `_新建轨道_0_2`) (`Timeline|时间轴_1`)
                              (:`Update`
                                (`MaterialInstanceDynamic.SetScalarParameterValue` _returnvalue_4 "Top" (`KismetMathLibrary.Lerp` 100.0 0.3 `_新建轨道_0_2`)))
                              (:`Finished`
                                ;[1 1 1] 判断是否是第二座塔（需要旋转）
                                (if (not (!= _hand_count 1))
                                  (bind _outactors_10 (`GameplayStatics.GetAllActorsOfClass` "/Game/JadeCiderquist/BluePrint/BP_DaoGuangTa.BP_DaoGuangTa_C"))
                                  (if (`/Game/JadeCiderquist/BluePrint/BP_DaoGuangTa.Complete` (`|GetArrayItem` _outactors_10 _hand_count))
                                    _
                                    (else
                                      (goto _label_6 :!via `Open`))))
                                ;[1 1 1] 主塔播放特效信号
                                (bind _outactors_11 (`GameplayStatics.GetAllActorsOfClass` "/Game/JadeCiderquist/BluePrint/BP_MainBuilding.BP_MainBuilding_C" :!label _label_3))
                                (bind _output_9 (`|GetArrayItem` _outactors_11))
                                (set `/Game/JadeCiderquist/BluePrint/BP_MainBuilding.Count` (`self.Hand_Count`) _output_9)
                                (message `/Game/JadeCiderquist/BluePrint/BI_OpenBuilding.OpenBuilding` _output_9))))))
                      (bind _output_get (set `/Game/AFCore/Examples/Pawns/VR/BP_Pawn_VR_Char_Example_HandsOn.Fire_Count` (- (stale _output_get) 3) _output)))
                    (:`then_2`
                      ;[1 1 1] 灯光变亮
                      (bind (_array_element _array_index) (`/Game/AFCore/Libraries/MLib_Actor_Macros.ForEachLoopWithDelay` _spot_light 6.0 :!label _label_4)
                        (:`LoopBody`
                          (bind (_direction_3 `_新建轨道_0_3`) (`Timeline|时间轴_2`)
                            (:`Update`
                              (`LightComponent.SetIntensity` (`Light.LightComponent` (`|GetArrayItem` _spot_light _array_index)) (`KismetMathLibrary.Lerp` 0.0 300.0 `_新建轨道_0_3`))))))))))
              (elif (== _hand_count_2 1)
                (`/Engine/EditorBlueprintResources/StandardMacros.DoOnce` false
                  (:`Completed`
                    (`|ExecutionSequence`
                      (:`then_0`
                        ;[1 1 1] 加速带引导
                        (bind _outactors_12 (`GameplayStatics.GetAllActorsOfClassWithTag` "/Game/Dangcl/Blueprint/A10Building.A10Building_C" "JiaSu1"))
                        (`SceneComponent.SetVisibility` (`/Game/Dangcl/Blueprint/A10Building.SM_YinDaoQi` (`|GetArrayItem` _outactors_12)) true false)
                        ;[1 1 1] 隐藏球体引导关闭
                        (bind _outactors_13 (`GameplayStatics.GetAllActorsOfClassWithTag` "/Game/JadeCiderquist/BluePrint/BP_DaoGuangTa.BP_DaoGuangTa_C" "TA1"))
                        (`SceneComponent.SetVisibility` (`/Game/JadeCiderquist/BluePrint/BP_DaoGuangTa.YinDao_Sphere` (`|GetArrayItem` _outactors_13)) false false)
                        ;[1 1 1] 点亮第二座塔插入钥匙引导
                        (bind _outactors_14 (`GameplayStatics.GetAllActorsOfClassWithTag` "/Game/JadeCiderquist/BluePrint/BP_DaoGuangTa.BP_DaoGuangTa_C" "TA1"))
                        (if (`/Game/JadeCiderquist/BluePrint/BP_DaoGuangTa.Open_Ket` (`|GetArrayItem` _outactors_14))
                          (goto _label_2)
                          (else
                            (`|ExecutionSequence`
                              (:`then_0`
                                (goto _label_2))
                              (:`then_1`
                                (`KismetSystemLibrary.Delay` 8.0)
                                (bind _outactors_15 (`GameplayStatics.GetAllActorsOfClass` "/Game/AFCore/Examples/Pawns/VR/BP_Pawn_VR_Char_Example_HandsOn.BP_Pawn_VR_Char_Example_HandsOn_C"))
                                (bind _wbp_keyta (`/Game/AFCore/Examples/Pawns/VR/BP_Pawn_VR_Char_Example_HandsOn.WBP_KeyTA` (`|GetArrayItem` _outactors_15)))
                                (`SceneComponent.SetVisibility` _wbp_keyta true false)
                                (`KismetSystemLibrary.Delay` 8.0)
                                (`SceneComponent.SetVisibility` _wbp_keyta false false))))))
                      (:`then_1`
                        (goto _label_4)))))
                (else
                  (goto _label_2))))))
        (else
          (`MaterialInstanceDynamic.SetVectorParameterValue` (`self.DynMaterial`) "color" (struct :`G` 0.115486 :`B` 0.255208 :`A` 1.0)))))))

(event `self.Shark_Sphere.OnComponentBeginOverlap`
  (params (OverlappedComponent :type "PrimitiveComponent Object Reference") (OtherActor :type "Actor Object Reference") (OtherComp :type "PrimitiveComponent Object Reference") (OtherBodyIndex :type Integer) (bFromSweep :type Boolean) (SweepResult :type "HitResult Structure (by ref)"))
  ;[1 1 1] 设置鲨鱼球体视野/
  (cast `/Game/AFCore/Examples/Pawns/VR/BP_Pawn_VR_Char_Example_HandsOn` OtherActor)
  (bind _outactors (`GameplayStatics.GetAllActorsOfClass` "/Game/AFCore/Examples/Pawns/VR/BP_Pawn_VR_Char_Example_HandsOn.BP_Pawn_VR_Char_Example_HandsOn_C"))
  (`SphereComponent.SetSphereRadius` (`/Game/AFCore/Examples/Pawns/VR/BP_Pawn_VR_Char_Example_HandsOn.Sharke_Sphere` (`|GetArrayItem` _outactors)) 0.0 true)
  (`/Engine/EditorBlueprintResources/StandardMacros.DoOnce` false :!label _label_5
    (:`Completed`
      (`UserWidget.AddToViewport` (`self.W_JiHuo`) 0)
      (goto _label :!via `Open`))))

(event `self.Shark_Sphere.OnComponentEndOverlap`
  (params (OverlappedComponent :type "PrimitiveComponent Object Reference") (OtherActor :type "Actor Object Reference") (OtherComp :type "PrimitiveComponent Object Reference") (OtherBodyIndex :type Integer))
  ;[1 1 1] 设置鲨鱼球体视野/
  (cast `/Game/AFCore/Examples/Pawns/VR/BP_Pawn_VR_Char_Example_HandsOn` OtherActor)
  (bind _outactors (`GameplayStatics.GetAllActorsOfClass` "/Game/AFCore/Examples/Pawns/VR/BP_Pawn_VR_Char_Example_HandsOn.BP_Pawn_VR_Char_Example_HandsOn_C"))
  (`SphereComponent.SetSphereRadius` (`/Game/AFCore/Examples/Pawns/VR/BP_Pawn_VR_Char_Example_HandsOn.Sharke_Sphere` (`|GetArrayItem` _outactors)) 180.0 true)
  (`|ExecutionSequence`
    (:`then_0`
      (`Widget.RemoveFromParent` (`self.W_JiHuo`))
      (goto _label :!via `Close`))
    (:`then_1`
      (goto _label_5 :!via `Reset`))))

(event `/Game/JadeCiderquist/BluePrint/BI_OpenBuilding.Com_TA`
  (`/Engine/EditorBlueprintResources/StandardMacros.DoOnce` false
    (:`Completed`
      (`/Engine/EditorBlueprintResources/StandardMacros.Gate` true :!label _label_6
        (:`Exit`
          (goto _label_3))))))

(fn `UserConstructionScript`
  (`SceneComponent.SetVisibility` (`self.SM_YinDaoQi`) (`self.引导`) false)
  (`SphereComponent.SetSphereRadius` (`self.Shark_Sphere`) (`self.Shark_Radius`) true))