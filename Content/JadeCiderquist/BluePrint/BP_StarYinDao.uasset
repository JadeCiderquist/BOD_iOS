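; BP_StarYinDao is an interactable guide actor that shows a Text widget while the VR example pawn is nearby.
; It creates the widget on BeginPlay, and its sphere trigger, sized by InSphereRadius in the construction script, adds or removes it on overlap.
; A DoOnce prevents repeat adds, and a Gate lets the interact event (E key, per comment) remove the widget and destroy the actor only while in range.
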(event `self.ReceiveBeginPlay`
  (bind _returnvalue (`|CreateWidget` (`self.Text`) (`GameplayStatics.GetPlayerController` 0)))
  (set `self.W_Var` _returnvalue))

(event `/Game/JadeCiderquist/BluePrint/BI_OpenBuilding.Open/Interacte`
  ;[1 1 1] 按E激活
  (`/Engine/EditorBlueprintResources/StandardMacros.Gate` true :!label _label
    (:`Exit`
      (`Widget.RemoveFromParent` (`self.W_Var`))
      (`self.K2_DestroyActor`))))

(event `self.Sphere.OnComponentBeginOverlap`
  (params (OverlappedComponent :type "PrimitiveComponent Object Reference") (OtherActor :type "Actor Object Reference") (OtherComp :type "PrimitiveComponent Object Reference") (OtherBodyIndex :type Integer) (bFromSweep :type Boolean) (SweepResult :type "HitResult Structure (by ref)"))
  (cast `/Game/AFCore/Examples/Pawns/VR/BP_Pawn_VR_Char_Example_HandsOn` OtherActor)
  (`/Engine/EditorBlueprintResources/StandardMacros.DoOnce` false :!label _label_2
    (:`Completed`
      (`UserWidget.AddToViewport` (`self.W_Var`) 0)
      (goto _label :!via `Open`))))

(event `self.Sphere.OnComponentEndOverlap`
  (params (OverlappedComponent :type "PrimitiveComponent Object Reference") (OtherActor :type "Actor Object Reference") (OtherComp :type "PrimitiveComponent Object Reference") (OtherBodyIndex :type Integer))
  (cast `/Game/AFCore/Examples/Pawns/VR/BP_Pawn_VR_Char_Example_HandsOn` OtherActor)
  (`Widget.RemoveFromParent` (`self.W_Var`))
  (`|ExecutionSequence`
    (:`then_0`
      (goto _label :!via `Close`))
    (:`then_1`
      (goto _label_2 :!via `Reset`))))

(fn `UserConstructionScript`
  (`SphereComponent.SetSphereRadius` (`self.Sphere`) (`self.In Sphere Radius`) true))