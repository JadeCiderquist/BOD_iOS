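; BP_magazine is an ammo magazine pickup for the VR pawn that refills the pistol.
; Sphere overlap opens a gate for the interact event and shrinks the pawn's SharkeSphere detection radius to zero, restoring it on exit.
; Interacting plays a sound, hides the clip components and BP_human02's SMYinDaoQi, and sets Pistol ammo, finding actors by class.
; It briefly shows the pawn's magazine notice widget, then destroys itself.
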(event `self.Comp_Grab.Grab_ActorPickedUp`
  (params (GrabbingPawn :type "/Game/AFCore/Blueprints/Pawn/BP_Pawn_Base Object Reference") (GrabbingActor :type "Actor Object Reference")))

(event `/Game/JadeCiderquist/BluePrint/BI_OpenBuilding.Open/Interacte`
  (`/Engine/EditorBlueprintResources/StandardMacros.Gate` true :!label _label
    (:`Exit`
      (`GameplayStatics.PlaySound2D` "/Game/JadeCiderquist/Sound/Gun_get.Gun_get" 1.0 1.0 0.0 null null)
      (bind _outactors (`GameplayStatics.GetAllActorsOfClass` "/Game/Dangcl/Blueprint/BP_human02.BP_human02_C"))
      (`SceneComponent.SetVisibility` (`self.CartridgeClip_L1`) false false)
      (`SceneComponent.SetVisibility` (`self.CartridgeClip_L2`) false false)
      (`SceneComponent.SetVisibility` (`self.CartridgeClip_L3`) false false)
      (`SceneComponent.SetVisibility` (`self.CartridgeClip_L`) false false)
      (`SceneComponent.SetVisibility` (`/Game/Dangcl/Blueprint/BP_human02.SM_YinDaoQi` (`|GetArrayItem` _outactors)) false false)
      ;[1 1 1] 设置子弹为10发
      (bind _outactors_2 (`GameplayStatics.GetAllActorsOfClass` "/Game/JadeCiderquist/Gun/Blueprints/Pistol.Pistol_C"))
      (bind _output (`|GetArrayItem` _outactors_2))
      (set `/Game/JadeCiderquist/Gun/Blueprints/Pistol.ZD_Max` 10 _output)
      (set `/Game/JadeCiderquist/Gun/Blueprints/Pistol.ZD_Count` 10 _output)
      ;[1 1 1] 提示获得弹夹
      (bind _outactors_3 (`GameplayStatics.GetAllActorsOfClass` "/Game/AFCore/Examples/Pawns/VR/BP_Pawn_VR_Char_Example_HandsOn.BP_Pawn_VR_Char_Example_HandsOn_C"))
      (bind _wbp_danjia (`/Game/AFCore/Examples/Pawns/VR/BP_Pawn_VR_Char_Example_HandsOn.WBP_DanJia` (`|GetArrayItem` _outactors_3)))
      (`SceneComponent.SetVisibility` _wbp_danjia true false)
      (`KismetSystemLibrary.Delay` 5.0)
      (`SceneComponent.SetVisibility` _wbp_danjia false false)
      (`self.K2_DestroyActor`))))

(event `self.Sphere.OnComponentBeginOverlap`
  (params (OverlappedComponent :type "PrimitiveComponent Object Reference") (OtherActor :type "Actor Object Reference") (OtherComp :type "PrimitiveComponent Object Reference") (OtherBodyIndex :type Integer) (bFromSweep :type Boolean) (SweepResult :type "HitResult Structure (by ref)"))
  ;[1 1 1] 设置角色鲨鱼检测球体半径/
  (bind _asbp_pawn_vr_char_example_hands_on (cast `/Game/AFCore/Examples/Pawns/VR/BP_Pawn_VR_Char_Example_HandsOn` OtherActor))
  (`SphereComponent.SetSphereRadius` (`/Game/AFCore/Examples/Pawns/VR/BP_Pawn_VR_Char_Example_HandsOn.Sharke_Sphere` _asbp_pawn_vr_char_example_hands_on) 0.0 true)
  (goto _label :!via `Open`))

(event `self.Sphere.OnComponentEndOverlap`
  (params (OverlappedComponent :type "PrimitiveComponent Object Reference") (OtherActor :type "Actor Object Reference") (OtherComp :type "PrimitiveComponent Object Reference") (OtherBodyIndex :type Integer))
  ;[1 1 1] 设置角色鲨鱼检测球体半径/
  (bind _asbp_pawn_vr_char_example_hands_on (cast `/Game/AFCore/Examples/Pawns/VR/BP_Pawn_VR_Char_Example_HandsOn` OtherActor))
  (`SphereComponent.SetSphereRadius` (`/Game/AFCore/Examples/Pawns/VR/BP_Pawn_VR_Char_Example_HandsOn.Sharke_Sphere` _asbp_pawn_vr_char_example_hands_on) 180.0 true)
  (goto _label :!via `Close`))

(fn `UserConstructionScript`)