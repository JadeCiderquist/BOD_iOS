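; BP_BOX_OpenLight is a one-shot trigger box that lights up a set of spotlights when the VR pawn enters it.
; On BeginPlay it sets every light in the SpotLight array to zero intensity.
; The first overlap by BP_Pawn_VR_Char_Example_HandsOn passes a DoOnce, then a delayed loop steps through the lights.
; Each step restarts one shared timeline that lerps the current light up to the target intensity, producing a staggered fade-in.
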(event `self.ReceiveBeginPlay`
  (bind _spot_light (`self.Spot_Light`))
  ;[1 1 1] 开始运行灯光关闭
  (bind (_array_element _array_index) (`/Game/AFCore/Libraries/MLib_Actor_Macros.ForEachLoopWithDelay` _spot_light)
    (:`LoopBody`
      (`LightComponent.SetIntensity` (`Light.LightComponent` (`|GetArrayItem` _spot_light _array_index)) 0.0))))

(event `self.Box.OnComponentBeginOverlap`
  (params (OverlappedComponent :type "PrimitiveComponent Object Reference") (OtherActor :type "Actor Object Reference") (OtherComp :type "PrimitiveComponent Object Reference") (OtherBodyIndex :type Integer) (bFromSweep :type Boolean) (SweepResult :type "HitResult Structure (by ref)"))
  (bind _spot_light (`self.Spot_Light`))
  (cast `/Game/AFCore/Examples/Pawns/VR/BP_Pawn_VR_Char_Example_HandsOn` OtherActor)
  (`/Engine/EditorBlueprintResources/StandardMacros.DoOnce` false
    (:`Completed`
      ;[1 1 1] 灯光变亮
      (bind (_array_element _array_index) (`/Game/AFCore/Libraries/MLib_Actor_Macros.ForEachLoopWithDelay` _spot_light 3.0)
        (:`LoopBody`
          (bind (_direction `_新建轨道_0`) (`Timeline|时间轴_0` :!via `PlayFromStart`)
            (:`Update`
              (`LightComponent.SetIntensity` (`Light.LightComponent` (`|GetArrayItem` _spot_light _array_index)) (`KismetMathLibrary.Lerp` 0.0 (`self.灯光强度`) `_新建轨道_0`)))))))))

(fn `UserConstructionScript`)