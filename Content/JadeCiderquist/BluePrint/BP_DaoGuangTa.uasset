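; Light-guide tower puzzle actor for VR; the Open/Interacte event, gated to the player being inside its shark detection sphere, triggers it.
; For Count 1, a timeline yaws the mechanism, moves TALight with ArrowLight, plays a door sound, then notifies BP_TaHand actors.
; Entering the sphere zeroes the pawn's SharkeSphere radius and hides the guide sphere, which Tick periodically pulses.
; Construction passes Count to linked hand and light when SetTA is set.
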(event `self.ReceiveBeginPlay`
  (`PrimitiveComponent.SetCollisionEnabled` (`self.MechanismA_Mechanism03_F`) "NoCollision"))

(event `self.ReceiveTick`
  (params (DeltaSeconds :type "Float (single-precision)"))
  (bind _yindao_sphere (`self.YinDao_Sphere`))
  ;[1 1 1] 引导球
  (`KismetSystemLibrary.Delay` 10.0)
  (bind (_direction `_新建轨道_0`) (`Timeline|时间轴_0` :!via `PlayFromStart`)
    (:`Update`
      (`SceneComponent.SetRelativeScale3D` _yindao_sphere (`KismetMathLibrary.Conv_DoubleToVector` (`KismetMathLibrary.Lerp` 0.0 300.0 `_新建轨道_0`))))
    (:`Finished`
      (`SceneComponent.SetRelativeScale3D` _yindao_sphere (0.0 0.0 0.0)))))

(event `/Game/JadeCiderquist/BluePrint/BI_OpenBuilding.Open/Interacte`
  (bind _arrow_light (`self.Arrow_Light`))
  (`/Engine/EditorBlueprintResources/StandardMacros.Gate` true :!label _label
    (:`Exit`
      (if (== (`self.Count`) 1)
        ;[1 1 1] 自动旋转-40
        (set `self.Complete` true)
        (bind (_direction `_新建轨道_0`) (`Timeline|时间轴_1`)
          (:`Update`
            (`SceneComponent.K2_SetRelativeRotation` (`self.MechanismA_Mechanism02_F`) (`KismetMathLibrary.MakeRotator` 0.0 0.0 (`KismetMathLibrary.Lerp` 0.0 -40.0 `_新建轨道_0`)) false false)
            (`SceneComponent.K2_SetWorldLocationAndRotation` (`Actor.RootComponent` (`self.TA_Light`)) (`SceneComponent.K2_GetComponentLocation` _arrow_light) (`SceneComponent.K2_GetComponentRotation` _arrow_light) false false)
            (`/Engine/EditorBlueprintResources/StandardMacros.DoOnce` false
              (:`Completed`
                (`GameplayStatics.PlaySound2D` "/Game/JadeCiderquist/Sound/Door_open.Door_open" 1.0 1.0 0.0 null null))))
          (:`Finished`
            (bind _outactors (`GameplayStatics.GetAllActorsOfClass` "/Game/JadeCiderquist/BluePrint/BP_TaHand.BP_TaHand_C"))
            (message `/Game/JadeCiderquist/BluePrint/BI_OpenBuilding.Com_TA` _outactors)))))))

(event `self.Shark_Sphere.OnComponentBeginOverlap`
  (params (OverlappedComponent :type "PrimitiveComponent Object Reference") (OtherActor :type "Actor Object Reference") (OtherComp :type "PrimitiveComponent Object Reference") (OtherBodyIndex :type Integer) (bFromSweep :type Boolean) (SweepResult :type "HitResult Structure (by ref)"))
  ;[1 1 1] 设置角色鲨鱼检测球体半径
  (bind _asbp_pawn_vr_char_example_hands_on (cast `/Game/AFCore/Examples/Pawns/VR/BP_Pawn_VR_Char_Example_HandsOn` OtherActor))
  (`SphereComponent.SetSphereRadius` (`/Game/AFCore/Examples/Pawns/VR/BP_Pawn_VR_Char_Example_HandsOn.Sharke_Sphere` _asbp_pawn_vr_char_example_hands_on) 0.0 true)
  (`SceneComponent.SetVisibility` (`self.YinDao_Sphere`) false false)
  (goto _label :!via `Open`))

(event `self.Comp_Drag.DragStateChanged_Constant`
  (params (SourceInfo :type "/Game/AFCore/Structs/Struct_Component_SourceInfo Structure") (Name :type Name) (Distance :type "Float (double-precision)") (Procent :type "Float (double-precision)") (Velocity :type "Float (double-precision)")))

(event `self.Shark_Sphere.OnComponentEndOverlap`
  (params (OverlappedComponent :type "PrimitiveComponent Object Reference") (OtherActor :type "Actor Object Reference") (OtherComp :type "PrimitiveComponent Object Reference") (OtherBodyIndex :type Integer))
  ;[1 1 1] 设置角色鲨鱼检测球体半径
  (bind _asbp_pawn_vr_char_example_hands_on (cast `/Game/AFCore/Examples/Pawns/VR/BP_Pawn_VR_Char_Example_HandsOn` OtherActor))
  (`SphereComponent.SetSphereRadius` (`/Game/AFCore/Examples/Pawns/VR/BP_Pawn_VR_Char_Example_HandsOn.Sharke_Sphere` _asbp_pawn_vr_char_example_hands_on) 180.0 true)
  (goto _label :!via `Close`))

(fn `UserConstructionScript`
  (bind _count (`self.Count`))
  (if (`self.Set_TA`)
    (set `/Game/JadeCiderquist/BluePrint/BP_TaHand.Hand_Count` _count (`self.Ta_Hand`))
    (set `/Game/JadeCiderquist/BluePrint/BP_GuangShu.Light_Count` _count (`self.TA_Light`))
    (`SceneComponent.K2_SetRelativeRotation` (`self.MechanismA_Mechanism01_F`) (`self.Rotation`) false false)
    (`SceneComponent.SetVisibility` (`self.SM_YinDaoQi`) (`self.引导`) false)
    (`SphereComponent.SetSphereRadius` (`self.Shark_Sphere`) (`self.Shark_Radius`) true)))