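; BP_Xuanwo is a whirlpool actor that acts as a level exit for the VR player.
; Its Niagara vortex color starts transparent at BeginPlay, and the ComXuanWo event fades it in via a timeline.
; When the VR pawn overlaps the capsule, the actor disables movement and plays haptics on both hands.
; A second timeline dims the underwater parameter collection's Light, with a delay off its update opening the target level.
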(event `self.ReceiveBeginPlay`
  (bind (_color_r _color_g _color_b) (break `LinearColor` (`self.Color`)))
  (`NiagaraComponent.SetVariableLinearColor` (`self.NS_Vortex`) "XW_Color" (`KismetMathLibrary.MakeColor` _color_r _color_g _color_b 0.0)))

(event `/Game/JadeCiderquist/BluePrint/BI_XuanWo.Com_XuanWo`
  (bind (_color_r _color_g _color_b) (break `LinearColor` (`self.Color`)))
  ;[0 0 0] 漩涡出现
  (bind (_direction `_新建轨道_0`) (`Timeline|时间轴_0`)
    (:`Update`
      (`NiagaraComponent.SetVariableLinearColor` (`self.NS_Vortex`) "XW_Color" (`KismetMathLibrary.MakeColor` _color_r _color_g _color_b (`KismetMathLibrary.Lerp` 0.0 1.0 `_新建轨道_0`))))))

(event `self.ReceiveTick`
  (params (DeltaSeconds :type "Float (single-precision)"))
  ;[0 0 0] 漩涡旋转
)

(event `self.Capsule.OnComponentBeginOverlap`
  (params (OverlappedComponent :type "PrimitiveComponent Object Reference") (OtherActor :type "Actor Object Reference") (OtherComp :type "PrimitiveComponent Object Reference") (OtherBodyIndex :type Integer) (bFromSweep :type Boolean) (SweepResult :type "HitResult Structure (by ref)"))
  (bind _returnvalue (`GameplayStatics.GetPlayerController` 0))
  (bind _asbp_pawn_vr_char_example_hands_on (cast `/Game/AFCore/Examples/Pawns/VR/BP_Pawn_VR_Char_Example_HandsOn` OtherActor))
  (set `/Game/AFCore/Examples/Pawns/VR/BP_Pawn_VR_Char_Example_HandsOn.if_Move` false _asbp_pawn_vr_char_example_hands_on)
  (`PlayerController.PlayHapticEffect` _returnvalue "/Game/JadeCiderquist/Gun/Haptics/PistolFireHapticEffect.PistolFireHapticEffect" "Left" 1.0 false)
  (`PlayerController.PlayHapticEffect` _returnvalue "/Game/JadeCiderquist/Gun/Haptics/PistolFireHapticEffect.PistolFireHapticEffect" "Right" 1.0 false)
  ;[0 0 0] 渐渐变黑
  (bind (_direction `_新建轨道_0`) (`Timeline|时间轴_1`)
    (:`Update`
      (`KismetMaterialLibrary.SetScalarParameterValue` "/Game/JadeCiderquist/Material/Underwater/MP_UnderWater.MP_UnderWater" "Light" (`KismetMathLibrary.Lerp` 1.0 0.0 `_新建轨道_0`))
      (`KismetSystemLibrary.Delay` 4.0)
      (`GameplayStatics.OpenLevelBySoftObjectPtr` (`self.Level`)))))

(fn `UserConstructionScript`
  (`NiagaraComponent.SetVariableLinearColor` (`self.NS_Vortex`) "XW_Color" (`self.Color`)))