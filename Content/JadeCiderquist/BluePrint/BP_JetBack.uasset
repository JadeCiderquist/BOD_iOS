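; BP_JetBack is a grabbable jetpack pickup that unlocks the jet ability for the VR player character.
; On grab, it finds the first BP_Pawn_VR_Char_Example_HandsOn in the level, sets its GetJetBack flag, and shows its speed-up widget and watch.
; It then hides its own backpack and SMYinDaoQi components in game.
; The sphere overlap only casts to the pawn and takes no further action.
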(event `self.Comp_Grab.Grab_ActorPickedUp`
  (params (GrabbingPawn :type "/Game/AFCore/Blueprints/Pawn/BP_Pawn_Base Object Reference") (GrabbingActor :type "Actor Object Reference"))
  ;[1 1 1] 开启喷气功能
  (bind _outactors (`GameplayStatics.GetAllActorsOfClass` "/Game/AFCore/Examples/Pawns/VR/BP_Pawn_VR_Char_Example_HandsOn.BP_Pawn_VR_Char_Example_HandsOn_C"))
  (bind _output (`|GetArrayItem` _outactors))
  (set `/Game/AFCore/Examples/Pawns/VR/BP_Pawn_VR_Char_Example_HandsOn.Get_JetBack` true _output)
  (`SceneComponent.SetVisibility` (`/Game/AFCore/Examples/Pawns/VR/BP_Pawn_VR_Char_Example_HandsOn.WBP_SpeedUp` _output) true false)
  (`SceneComponent.SetHiddenInGame` (`self.JetBackpack`) true false)
  (`SceneComponent.SetHiddenInGame` (`self.SM_YinDaoQi`) true false)
  ;[1 1 1] 显示手表
  (`SceneComponent.SetVisibility` (`/Game/AFCore/Examples/Pawns/VR/BP_Pawn_VR_Char_Example_HandsOn.Watch` _output) true false))

(event `self.Sphere.OnComponentBeginOverlap`
  (params (OverlappedComponent :type "PrimitiveComponent Object Reference") (OtherActor :type "Actor Object Reference") (OtherComp :type "PrimitiveComponent Object Reference") (OtherBodyIndex :type Integer) (bFromSweep :type Boolean) (SweepResult :type "HitResult Structure (by ref)"))
  (cast `/Game/AFCore/Examples/Pawns/VR/BP_Pawn_VR_Char_Example_HandsOn` OtherActor))

(fn `UserConstructionScript`)