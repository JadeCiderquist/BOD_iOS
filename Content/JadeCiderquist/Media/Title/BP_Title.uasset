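; BP_Title is an actor that plays a one-time title intro sequence once PlayTitle is set, then destroys itself.
; Timelines drive the Strenth parameter of a dynamic M_Title material on its Plane, then fade three texts in and out in turn, with sounds along the way.
; Steps chain through Delays on timeline Update pins, and BP_Xuanwo (whirlpool) is messaged before Text3.
; The Media playback and reset logic is unconnected.
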(event `self.ReceiveBeginPlay`)

(event `self.ReceiveTick`
  (params (DeltaSeconds :type "Float (single-precision)"))
  (if (`self.Play_Title`)
    (`/Engine/EditorBlueprintResources/StandardMacros.DoOnce` false
      (:`Completed`
        (`GameplayStatics.PlaySound2D` "/Game/JadeCiderquist/Sound/Title_appearance0.Title_appearance0" 1.0 1.0 0.0 null null)
        (bind (_direction `_新建轨道_0`) (`Timeline|时间轴_7`)
          (:`Update`
            (`MaterialInstanceDynamic.SetScalarParameterValue` (`self.Material`) "Strenth" (`KismetMathLibrary.Lerp` 0.8 0.0 `_新建轨道_0`)))
          (:`Finished`
            (`KismetSystemLibrary.Delay` 1.0)
            ;[1 1 1] 标题结束
            (bind (_direction_2 `_新建轨道_0_2`) (`Timeline|时间轴_0`)
              (:`Update`
                (`MaterialInstanceDynamic.SetScalarParameterValue` (`self.Material`) "Strenth" (`KismetMathLibrary.Lerp` 0.0 1.0 `_新建轨道_0_2`))
                (`KismetSystemLibrary.Delay` 2.0)
                ;[1 1 1] Text1
                (`GameplayStatics.PlaySound2D` "/Game/JadeCiderquist/Sound/Sound_HaiNan.Sound_HaiNan" 1.0 1.0 0.0 null null)
                (bind (_direction_3 `_新建轨道_0_3`) (`Timeline|时间轴_1`)
                  (:`Update`
                    (`WidgetComponent.SetTintColorAndOpacity` (`self.Text1`) (make `LinearColor` 1.0 1.0 1.0 (`KismetMathLibrary.Lerp` 0.0 0.5 `_新建轨道_0_3`)))
                    (`KismetSystemLibrary.Delay` (`self.Text_Time`))
                    (bind (_direction_4 `_新建轨道_0_4`) (`Timeline|时间轴_2`)
                      (:`Update`
                        (`WidgetComponent.SetTintColorAndOpacity` (`self.Text1`) (make `LinearColor` 1.0 1.0 1.0 (`KismetMathLibrary.Lerp` 0.5 0.0 `_新建轨道_0_4`)))
                        (`KismetSystemLibrary.Delay` (`self.Text_Time`))
                        ;[1 1 1] Text2
                        (`|ExecutionSequence`
                          (:`then_0`
                            (bind (_direction_5 `_新建轨道_0_5`) (`Timeline|时间轴_3`)
                              (:`Update`
                                (`WidgetComponent.SetTintColorAndOpacity` (`self.Text2`) (make `LinearColor` 1.0 1.0 1.0 (`KismetMathLibrary.Lerp` 0.0 0.5 `_新建轨道_0_5`)))
                                (`KismetSystemLibrary.Delay` (`self.Text_Time`))
                                (bind (_direction_6 `_新建轨道_0_6`) (`Timeline|时间轴_4`)
                                  (:`Update`
                                    (`WidgetComponent.SetTintColorAndOpacity` (`self.Text2`) (make `LinearColor` 1.0 1.0 1.0 (`KismetMathLibrary.Lerp` 0.5 0.0 `_新建轨道_0_6`)))
                                    (`KismetSystemLibrary.Delay` (`self.Text_Time`))
                                    ;[1 1 1] 漩涡
                                    (bind _outactors (`GameplayStatics.GetAllActorsOfClass` "/Game/JadeCiderquist/BluePrint/BP_Xuanwo.BP_Xuanwo_C"))
                                    (message `/Game/JadeCiderquist/BluePrint/BI_XuanWo.Com_XuanWo` _outactors)
                                    ;[1 1 1] Text3
                                    (bind (_direction_7 `_新建轨道_0_7`) (`Timeline|时间轴_5`)
                                      (:`Update`
                                        (`WidgetComponent.SetTintColorAndOpacity` (`self.Text3`) (make `LinearColor` 1.0 1.0 1.0 (`KismetMathLibrary.Lerp` 0.0 0.5 `_新建轨道_0_7`)))
                                        (`KismetSystemLibrary.Delay` (`self.Text_Time`))
                                        (bind (_direction_8 `_新建轨道_0_8`) (`Timeline|时间轴_6`)
                                          (:`Update`
                                            (`WidgetComponent.SetTintColorAndOpacity` (`self.Text3`) (make `LinearColor` 1.0 1.0 1.0 (`KismetMathLibrary.Lerp` 0.5 0.0 `_新建轨道_0_8`)))
                                            (`KismetSystemLibrary.Delay` (`self.Text_Time`))
                                            (`self.K2_DestroyActor`))))))))))
                          (:`then_1`
                            (`/Engine/EditorBlueprintResources/StandardMacros.DoOnce` false
                              (:`Completed`
                                (`GameplayStatics.PlaySound2D` "/Game/JadeCiderquist/Sound/Sound_XuanWo.Sound_XuanWo" 1.0 1.0 0.0 null null)))))))))))))))))

(fn `UserConstructionScript`
  (bind _returnvalue (`PrimitiveComponent.CreateDynamicMaterialInstance` (`self.Plane`) 0 "/Game/JadeCiderquist/Media/Title/M_Title.M_Title" "None"))
  (set `self.Material` _returnvalue))