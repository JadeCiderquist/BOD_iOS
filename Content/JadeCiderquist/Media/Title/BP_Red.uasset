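; BP_Red is a title actor that shows three texts in sequence, then destroys itself.
; On BeginPlay, six chained timelines fade each text's tint alpha up to half opacity and back to zero, separated by configurable delays, with separate timing for the last text.
; Each next step hangs off the previous timeline's Update through a Delay, not Finished.
; The construction script stores a dynamic M_Title material for the Plane, unused in the event graph.
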(event `self.ReceiveBeginPlay`
  ;[1 1 1] Text1
  (bind (_direction `_新建轨道_0`) (`Timeline|时间轴_1`)
    (:`Update`
      (`WidgetComponent.SetTintColorAndOpacity` (`self.Text1`) (make `LinearColor` 1.0 1.0 1.0 (`KismetMathLibrary.Lerp` 0.0 0.5 `_新建轨道_0`)))
      (`KismetSystemLibrary.Delay` (`self.Text_Time`))
      (bind (_direction_2 `_新建轨道_0_2`) (`Timeline|时间轴_2`)
        (:`Update`
          (`WidgetComponent.SetTintColorAndOpacity` (`self.Text1`) (make `LinearColor` 1.0 1.0 1.0 (`KismetMathLibrary.Lerp` 0.5 0.0 `_新建轨道_0_2`)))
          (`KismetSystemLibrary.Delay` (`self.Text_Time`))
          ;[1 1 1] Text2
          (bind (_direction_3 `_新建轨道_0_3`) (`Timeline|时间轴_3`)
            (:`Update`
              (`WidgetComponent.SetTintColorAndOpacity` (`self.Text2`) (make `LinearColor` 1.0 1.0 1.0 (`KismetMathLibrary.Lerp` 0.0 0.5 `_新建轨道_0_3`)))
              (`KismetSystemLibrary.Delay` (`self.Text_Time`))
              (bind (_direction_4 `_新建轨道_0_4`) (`Timeline|时间轴_4`)
                (:`Update`
                  (`WidgetComponent.SetTintColorAndOpacity` (`self.Text2`) (make `LinearColor` 1.0 1.0 1.0 (`KismetMathLibrary.Lerp` 0.5 0.0 `_新建轨道_0_4`)))
                  (`KismetSystemLibrary.Delay` (`self.Text_Time`))
                  ;[1 1 1] Text3
                  (bind (_direction_5 `_新建轨道_0_5`) (`Timeline|时间轴_5`)
                    (:`Update`
                      (`WidgetComponent.SetTintColorAndOpacity` (`self.Text3`) (make `LinearColor` 1.0 1.0 1.0 (`KismetMathLibrary.Lerp` 0.0 0.5 `_新建轨道_0_5`)))
                      (`KismetSystemLibrary.Delay` (`self.Text_Time_final`))
                      (bind (_direction_6 `_新建轨道_0_6`) (`Timeline|时间轴_6`)
                        (:`Update`
                          (`WidgetComponent.SetTintColorAndOpacity` (`self.Text3`) (make `LinearColor` 1.0 1.0 1.0 (`KismetMathLibrary.Lerp` 0.5 0.0 `_新建轨道_0_6`)))
                          (`KismetSystemLibrary.Delay` (`self.Text_Time_final`))
                          (`self.K2_DestroyActor`))))))))))))))

(fn `UserConstructionScript`
  (bind _returnvalue (`PrimitiveComponent.CreateDynamicMaterialInstance` (`self.Plane`) 0 "/Game/JadeCiderquist/Media/Title/M_Title.M_Title" "None"))
  (set `self.Material` _returnvalue))