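; VR pistol actor that auto-attaches to the player's right hand on overlap once the QianTing actor's OpenGun flag is set.
; A one-time timeline snap shows the gun UI, enables the pawn's shark-detection sphere and opens the firing gate.
; PShot spawns projectiles with effects and haptics, or signals empty ammo; reload logic is unconnected.
; Releasing disables shark detection and teleports the gun to the right controller after four seconds unless held.
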(event `self.Comp_Grab.Grab_ActorPickedUp`
  (params (GrabbingPawn :type "/Game/AFCore/Blueprints/Pawn/BP_Pawn_Base Object Reference") (GrabbingActor :type "Actor Object Reference")))

(event `self.Comp_Grab.Grab_ActorReleased`
  (params (ReleasingPawn :type "/Game/AFCore/Blueprints/Pawn/BP_Pawn_Base Object Reference") (ReleasingActor :type "Actor Object Reference") (LastRelease :type Boolean))
  (set `self.Pick_Up` false)
  (`|ExecutionSequence`
    (:`then_0`
      (`KismetSystemLibrary.Delay` 4.0)
      (if (not (`self.Pick_Up`))
        ;[1 1 1] 松开手枪后自动设置到右手
        (bind _outactors (`GameplayStatics.GetAllActorsOfClass` "/Game/AFCore/Examples/Pawns/VR/BP_Pawn_VR_Char_Example_HandsOn.BP_Pawn_VR_Char_Example_HandsOn_C"))
        (`self.K2_SetActorLocation` (`SceneComponent.K2_GetComponentLocation` (`/Game/AFCore/Blueprints/Pawn/VR/BP_Pawn_VR.MotionControllerRight` (`|GetArrayItem` _outactors))))))
    (:`then_1`
      ;[1 1 1] 丢枪，关闭鲨鱼检测碰撞
      (bind _outactors_2 (`GameplayStatics.GetAllActorsOfClass` "/Game/AFCore/Examples/Pawns/VR/BP_Pawn_VR_Char_Example_HandsOn.BP_Pawn_VR_Char_Example_HandsOn_C"))
      (`PrimitiveComponent.SetCollisionEnabled` (`/Game/AFCore/Examples/Pawns/VR/BP_Pawn_VR_Char_Example_HandsOn.Sharke_Sphere` (`|GetArrayItem` _outactors_2)) "NoCollision"))))

(event `/Game/JadeCiderquist/Gun/Blueprints/VRInteractionBPI.P_Shot`
  (bind _fx_shot (`self.Fx_Shot`))
  (bind _muzzlelocation (`self.MuzzleLocation`))
  (`/Engine/EditorBlueprintResources/StandardMacros.Gate` true :!label _label
    (:`Exit`
      (if (> (`self.ZD_Count`) 0)
        (`PlayerCameraManager.StartCameraShake` :`self` (`GameplayStatics.GetPlayerCameraManager` 0) :`ShakeClass` "/Game/JadeCiderquist/CameraSHake.CameraSHake_C" :`Scale` 0.1)
        (`ActorComponent.Deactivate` _fx_shot)
        (`ActorComponent.Activate` _fx_shot false)
        ;[1 1 1] 开枪减子弹数
        (bind _output_get (set `self.ZD_Count` (- (stale _output_get) 1)))
        (`GameplayStatics.PlaySound2D` "/Game/JadeCiderquist/Sound/Gun_Shot.Gun_Shot" 1.0 1.0 0.0 null null)
        ;[1 1 1] 生成子弹
        (`|SpawnActorFromClass` "/Game/JadeCiderquist/Gun/Blueprints/Projectile.Projectile_C" (`KismetMathLibrary.MakeTransform` (`SceneComponent.K2_GetComponentLocation` _muzzlelocation) (`SceneComponent.K2_GetComponentRotation` _muzzlelocation)) "Undefined" "OverrideRootScale" self (`GameplayStatics.GetPlayerPawn` 0))
        ;[1 1 1] 手机震动
        (`PlayerController.PlayDynamicForceFeedback` (`GameplayStatics.GetPlayerController` 0) 3.0 0.12 true true true true)
        (else
          ;[1 1 1] 没子弹了
          (`GameplayStatics.PlaySound2D` "/Game/JadeCiderquist/Sound/Gun_NoShot.Gun_NoShot" 1.0 1.0 0.0 null null)
          (`/Engine/EditorBlueprintResources/StandardMacros.DoOnce` false
            (:`Completed`
              (bind _outactors (`GameplayStatics.GetAllActorsOfClass` "/Game/AFCore/Examples/Pawns/VR/BP_Pawn_VR_Char_Example_HandsOn.BP_Pawn_VR_Char_Example_HandsOn_C"))
              (`SceneComponent.SetVisibility` (`/Game/AFCore/Examples/Pawns/VR/BP_Pawn_VR_Char_Example_HandsOn.WBP_NoShot` (`|GetArrayItem` _outactors)) true false))))))))

(event `self.Sphere.OnComponentBeginOverlap`
  (params (OverlappedComponent :type "PrimitiveComponent Object Reference") (OtherActor :type "Actor Object Reference") (OtherComp :type "PrimitiveComponent Object Reference") (OtherBodyIndex :type Integer) (bFromSweep :type Boolean) (SweepResult :type "HitResult Structure (by ref)"))
  ;[1 1 1] 手和枪重叠
  (bind _asbp_pawn_vr_char_example_hands_on (cast `/Game/AFCore/Examples/Pawns/VR/BP_Pawn_VR_Char_Example_HandsOn` OtherActor))
  (bind _outactors (`GameplayStatics.GetAllActorsOfClass` "/Game/WengZhiBo/Actor/QianTing.QianTing_C"))
  (if (`/Game/WengZhiBo/Actor/QianTing.Open_Gun` (`|GetArrayItem` _outactors))
    (`/Engine/EditorBlueprintResources/StandardMacros.DoOnce` false
      (:`Completed`
        (`|ExecutionSequence`
          (:`then_0`
            (`KismetSystemLibrary.Delay` 0.1)
            ;[1 1 1] 拾取枪支
            (`SceneComponent.SetVisibility` (`self.SM_YinDaoQi`) false false)
            (set `self.Pick_Once` true)
            (set `self.Pick_Up` true)
            ;[1 1 1] 拾取枪，开启鲨鱼检测碰撞
            (bind _outactors_2 (`GameplayStatics.GetAllActorsOfClass` "/Game/AFCore/Examples/Pawns/VR/BP_Pawn_VR_Char_Example_HandsOn.BP_Pawn_VR_Char_Example_HandsOn_C"))
            (`PrimitiveComponent.SetCollisionEnabled` (`/Game/AFCore/Examples/Pawns/VR/BP_Pawn_VR_Char_Example_HandsOn.Sharke_Sphere` (`|GetArrayItem` _outactors_2)) "QueryAndPhysics"))
          (:`then_1`
            (set `self.Pistol_Ts` (`self.GetTransform`))
            (set `self.Hand_Ts` (`SceneComponent.K2_GetComponentToWorld` (`/Game/AFCore/Examples/Pawns/VR/BP_Pawn_VR_Char_Example_HandsOn.RightSideArrowGun` _asbp_pawn_vr_char_example_hands_on)))
            ;[1 1 1] 靠近吸附
            (bind (_direction `_新建轨道_0`) (`Timeline|时间轴_1`)
              (:`Update`
                (bind (_returnvalue_location _returnvalue_rotation) (`KismetMathLibrary.BreakTransform` (`KismetMathLibrary.TLerp` (`self.Pistol_Ts`) (`self.Hand_Ts`) `_新建轨道_0`)))
                (`self.K2_SetActorTransform` (`KismetMathLibrary.MakeTransform` _returnvalue_location _returnvalue_rotation)))
              (:`Finished`
                (bind _outactors_3 (`GameplayStatics.GetAllActorsOfClass` "/Game/AFCore/Examples/Pawns/VR/BP_Pawn_VR_Char_Example_HandsOn.BP_Pawn_VR_Char_Example_HandsOn_C"))
                (bind _output (`|GetArrayItem` _outactors_3))
                (set `/Game/AFCore/Examples/Pawns/VR/BP_Pawn_VR_Char_Example_HandsOn.Pick_Gun` true _output)
                (`self.K2_AttachToComponent` self (`/Game/AFCore/Examples/Pawns/VR/BP_Pawn_VR_Char_Example_HandsOn.RightSideArrowGun` _output) "None" "SnapToTarget" "SnapToTarget" "SnapToTarget" true)
                (goto _label :!via `Open`))))
          (:`then_2`
            ;[1 1 1] 开枪UI
            (bind _returnvalue (`|CreateWidget` "/Game/JadeCiderquist/Widget/Button/W_Gun_Interaction.W_Gun_Interaction_C" (`GameplayStatics.GetPlayerController` 0)))
            (`UserWidget.AddToViewport` _returnvalue 0)))))))

(event `self.Comp_Grab.Grab_KeyInput`
  (params (MComp :type "/Game/AFCore/Blueprints/VR/MotionComponents/BP_MComp Object Reference") (Key :type "/Game/AFCore/Enums/Enum_Controller_Buttons Enum" :default "NewEnumerator1") (Set :type Boolean)))

(fn `UserConstructionScript`)