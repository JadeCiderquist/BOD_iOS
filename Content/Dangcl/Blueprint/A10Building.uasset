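; A10Building is an actor that acts as an acceleration trigger for the VR player pawn, with an optional guide mesh.
; When a BP_Pawn_VR_Char_Example_HandsOn overlaps its Capsule, it passes the Arrow's forward vector and a Speed value to the pawn's PAccelerationMessage, then hides the SMYinDaoQi guide mesh.
; The construction script sets that mesh's initial visibility from the 引导 (guide) flag.
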(event `self.Capsule.OnComponentBeginOverlap`
  (params (OverlappedComponent :type "PrimitiveComponent Object Reference") (OtherActor :type "Actor Object Reference") (OtherComp :type "PrimitiveComponent Object Reference") (OtherBodyIndex :type Integer) (bFromSweep :type Boolean) (SweepResult :type "HitResult Structure (by ref)"))
  (bind _asbp_pawn_vr_char_example_hands_on (cast `/Game/AFCore/Examples/Pawns/VR/BP_Pawn_VR_Char_Example_HandsOn` OtherActor))
  (message `/Game/AFCore/Examples/Pawns/VR/Bl_Pawn.P_acceleration` _asbp_pawn_vr_char_example_hands_on (`SceneComponent.GetForwardVector` (`self.Arrow`)) (`self.Speed`))
  (`SceneComponent.SetVisibility` (`self.SM_YinDaoQi`) false false))

(fn `UserConstructionScript`
  (`SceneComponent.SetVisibility` (`self.SM_YinDaoQi`) (`self.引导`) false))