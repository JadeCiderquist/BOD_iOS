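; BP_Plants03 is a cluster of vegetation meshes that grows into view when the VR hands-on pawn enters its capsule.
; Unless StartOn is set, BeginPlay scales all seven meshes to zero.
; The first overlap by that pawn passes a DoOnce and plays a timeline that lerps their shared scale up to full size.
; With StartOn set, the plants skip both the hiding and the growth.
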(event `self.ReceiveBeginPlay`
  (if (not (`self.Start_On`))
    (`SceneComponent.SetRelativeScale3D` (`self.Vegetation_05_F`) (0.0 0.0 0.0))
    (`SceneComponent.SetRelativeScale3D` (`self.Vegetation_06_F`) (0.0 0.0 0.0))
    (`SceneComponent.SetRelativeScale3D` (`self.Vegetation_05_F1`) (0.0 0.0 0.0))
    (`SceneComponent.SetRelativeScale3D` (`self.Vegetation_06_F1`) (0.0 0.0 0.0))
    (`SceneComponent.SetRelativeScale3D` (`self.Vegetation_06_F2`) (0.0 0.0 0.0))
    (`SceneComponent.SetRelativeScale3D` (`self.Vegetation_07_F`) (0.0 0.0 0.0))
    (`SceneComponent.SetRelativeScale3D` (`self.Vegetation_04_F`) (0.0 0.0 0.0))))

(event `self.Capsule.OnComponentBeginOverlap`
  (params (OverlappedComponent :type "PrimitiveComponent Object Reference") (OtherActor :type "Actor Object Reference") (OtherComp :type "PrimitiveComponent Object Reference") (OtherBodyIndex :type Integer) (bFromSweep :type Boolean) (SweepResult :type "HitResult Structure (by ref)"))
  (cast `/Game/AFCore/Examples/Pawns/VR/BP_Pawn_VR_Char_Example_HandsOn` OtherActor)
  (if (not (`self.Start_On`))
    (`/Engine/EditorBlueprintResources/StandardMacros.DoOnce` false
      (:`Completed`
        (bind (_direction `_新建轨道_0`) (`Timeline|时间轴_0` :!via `PlayFromStart`)
          (:`Update`
            (`SceneComponent.SetRelativeScale3D` (`self.Vegetation_05_F1`) (`KismetMathLibrary.Conv_DoubleToVector` (`KismetMathLibrary.Lerp` 0.0 1.0 `_新建轨道_0`)))
            (`SceneComponent.SetRelativeScale3D` (`self.Vegetation_04_F`) (`KismetMathLibrary.Conv_DoubleToVector` (`KismetMathLibrary.Lerp` 0.0 1.0 `_新建轨道_0`)))
            (`SceneComponent.SetRelativeScale3D` (`self.Vegetation_05_F`) (`KismetMathLibrary.Conv_DoubleToVector` (`KismetMathLibrary.Lerp` 0.0 1.0 `_新建轨道_0`)))
            (`SceneComponent.SetRelativeScale3D` (`self.Vegetation_06_F`) (`KismetMathLibrary.Conv_DoubleToVector` (`KismetMathLibrary.Lerp` 0.0 1.0 `_新建轨道_0`)))
            (`SceneComponent.SetRelativeScale3D` (`self.Vegetation_06_F1`) (`KismetMathLibrary.Conv_DoubleToVector` (`KismetMathLibrary.Lerp` 0.0 1.0 `_新建轨道_0`)))
            (`SceneComponent.SetRelativeScale3D` (`self.Vegetation_07_F`) (`KismetMathLibrary.Conv_DoubleToVector` (`KismetMathLibrary.Lerp` 0.0 1.0 `_新建轨道_0`)))
            (`SceneComponent.SetRelativeScale3D` (`self.Vegetation_06_F2`) (`KismetMathLibrary.Conv_DoubleToVector` (`KismetMathLibrary.Lerp` 0.0 1.0 `_新建轨道_0`)))))))))

(fn `UserConstructionScript`)