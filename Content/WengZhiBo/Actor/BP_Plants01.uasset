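; BP_Plants01 is a cluster of vegetation components with a point light that grows and lights up when the VR pawn walks into its capsule.
; Unless StartOn is set, BeginPlay scales the plants to zero and turns the light off.
; The first overlap by BP_Pawn_VR_Char_Example_HandsOn plays a timeline once, lerping plant scale to full and light intensity to its configured value.
; The construction script applies the exposed light settings and light function material.
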(event `self.ReceiveBeginPlay`
  (set `self.Vegetation` (`|MakeArray` (`self.Vegetation_06_F`) (`self.Vegetation_01_F`) (`self.Vegetation_03_F`) (`self.Vegetation_04_F`) (`self.Vegetation_05_F`) (`self.Vegetation_07_F`) (`self.Vegetation_05_F1`) (`self.Vegetation_07_F1`) (`self.Vegetation_04_F1`) (`self.Vegetation_06_F1`) (`self.Vegetation_06_F2`) (`self.Vegetation_07_F2`)))
  (if (not (`self.Start_On`))
    (`LightComponent.SetIntensity` (`self.PointLight`) 0.0)
    (for _array_element (`self.Vegetation`)
      (`SceneComponent.SetRelativeScale3D` _array_element (0.0 0.0 0.0)))))

(event `self.Capsule.OnComponentBeginOverlap`
  (params (OverlappedComponent :type "PrimitiveComponent Object Reference") (OtherActor :type "Actor Object Reference") (OtherComp :type "PrimitiveComponent Object Reference") (OtherBodyIndex :type Integer) (bFromSweep :type Boolean) (SweepResult :type "HitResult Structure (by ref)"))
  (cast `/Game/AFCore/Examples/Pawns/VR/BP_Pawn_VR_Char_Example_HandsOn` OtherActor)
  (if (not (`self.Start_On`))
    (`/Engine/EditorBlueprintResources/StandardMacros.DoOnce` false
      (:`Completed`
        (bind (_direction `_新建轨道_0`) (`Timeline|时间轴_0` :!via `PlayFromStart`)
          (:`Update`
            (`SceneComponent.SetRelativeScale3D` (`self.Vegetation_06_F`) (`KismetMathLibrary.Conv_DoubleToVector` (`KismetMathLibrary.Lerp` 0.0 1.0 `_新建轨道_0`)))
            (`SceneComponent.SetRelativeScale3D` (`self.Vegetation_03_F`) (`KismetMathLibrary.Conv_DoubleToVector` (`KismetMathLibrary.Lerp` 0.0 1.0 `_新建轨道_0`)))
            (`SceneComponent.SetRelativeScale3D` (`self.Vegetation_04_F`) (`KismetMathLibrary.Conv_DoubleToVector` (`KismetMathLibrary.Lerp` 0.0 1.0 `_新建轨道_0`)))
            (`SceneComponent.SetRelativeScale3D` (`self.Vegetation_05_F`) (`KismetMathLibrary.Conv_DoubleToVector` (`KismetMathLibrary.Lerp` 0.0 1.0 `_新建轨道_0`)))
            (`SceneComponent.SetRelativeScale3D` (`self.Vegetation_07_F`) (`KismetMathLibrary.Conv_DoubleToVector` (`KismetMathLibrary.Lerp` 0.0 1.0 `_新建轨道_0`)))
            (`SceneComponent.SetRelativeScale3D` (`self.Vegetation_05_F1`) (`KismetMathLibrary.Conv_DoubleToVector` (`KismetMathLibrary.Lerp` 0.0 1.0 `_新建轨道_0`)))
            (`SceneComponent.SetRelativeScale3D` (`self.Vegetation_01_F`) (`KismetMathLibrary.Conv_DoubleToVector` (`KismetMathLibrary.Lerp` 0.0 1.0 `_新建轨道_0`)))
            (`SceneComponent.SetRelativeScale3D` (`self.Vegetation_07_F1`) (`KismetMathLibrary.Conv_DoubleToVector` (`KismetMathLibrary.Lerp` 0.0 1.0 `_新建轨道_0`)))
            (`SceneComponent.SetRelativeScale3D` (`self.Vegetation_06_F1`) (`KismetMathLibrary.Conv_DoubleToVector` (`KismetMathLibrary.Lerp` 0.0 1.0 `_新建轨道_0`)))
            (`SceneComponent.SetRelativeScale3D` (`self.Vegetation_06_F2`) (`KismetMathLibrary.Conv_DoubleToVector` (`KismetMathLibrary.Lerp` 0.0 1.0 `_新建轨道_0`)))
            (`SceneComponent.SetRelativeScale3D` (`self.Vegetation_07_F2`) (`KismetMathLibrary.Conv_DoubleToVector` (`KismetMathLibrary.Lerp` 0.0 1.0 `_新建轨道_0`)))
            (`SceneComponent.SetRelativeScale3D` (`self.Vegetation_04_F1`) (`KismetMathLibrary.Conv_DoubleToVector` (`KismetMathLibrary.Lerp` 0.0 1.0 `_新建轨道_0`)))
            (`LightComponent.SetIntensity` (`self.PointLight`) (`KismetMathLibrary.Lerp` 0.0 (`self.强度`) `_新建轨道_0`))))))))

(fn `UserConstructionScript`
  (bind _pointlight (`self.PointLight`))
  (`LightComponent.SetIntensity` _pointlight (`self.强度`))
  (`PointLightComponent.SetSourceRadius` _pointlight (`self.源半径`))
  (`LocalLightComponent.SetAttenuationRadius` _pointlight (`self.衰减半径`))
  (`LightComponent.SetLightFunctionMaterial` _pointlight (`self.Light Function Material`)))